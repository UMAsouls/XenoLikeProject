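; BP_ArtSelectComponent tracks which Art is selected on a palette and resolves what using it triggers.
; SelectArt steps by direction, scanning forward only past slots unflagged in IsSet and keeping the current index if none is found.
; UseArt returns an offset Art index for side slots, or delegates the center slot to UseCenterArt.
; The center slot draws the weapon first, then yields the icon chosen via ChangeCenterArt, one type of which clears DrawWeapon.
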(event Custom|Initialize
  ;[0.15 0.15 0.15 0.5] Index初期化
  (Variables|Default|SetArtSelectIndex 2)
  (for _index (range 0 (Variables|Default|GetPaletteMaxIndex))
    (Utilities|Array|SetArrayElem (Variables|Default|GetIsSet) _index false)))

(event Custom|SelectArt
  (params (Direction :type Float%20%28double-precision%29))
  ;[0.15 0.15 0.15 0.5] アーツ選択処理
  (Variables|Default|SetSelectDirection (Math|Float|Truncate Direction))
  (Variables|Default|SetNextIndex (+ (Variables|Default|GetArtSelectIndex) (Variables|Default|GetSelectDirection)))
  (if (Utilities|Array|IsValidIndex (Variables|Default|GetIsSet) (Variables|Default|GetNextIndex))
    (while (not (Utilities|Array|Get(acopy) (Variables|Default|GetIsSet) (Variables|Default|GetNextIndex)))
      (Math|Integer|IncrementInt (Variables|Default|GetNextIndex)
        (:%20%20
          (if (not (Utilities|Array|IsValidIndex (Variables|Default|GetIsSet) (Variables|Default|GetNextIndex)))
            (Variables|Default|SetNextIndex (Variables|Default|GetArtSelectIndex))))))
    (Variables|Default|SetArtSelectIndex (Variables|Default|GetNextIndex))))

(event Custom|ChangeCenterArt
  (params (Direction :type Float%20%28double-precision%29))
  ;[0.15 0.15 0.15 0.5] 中央のアイコン変更
  (if (Utilities|Array|IsValidIndex (Variables|Default|GetCenterArts) (+ (Math|Float|Truncate Direction) (Variables|Default|GetCenterArtIndex)))
    (Variables|Default|SetCenterArtIndex (+ (Math|Float|Truncate Direction) (Variables|Default|GetCenterArtIndex)))))

(event EventBeginPlay)

(event EventTick
  (params (DeltaSeconds :type Float%20%28single-precision%29)))

(fn UseArt
  (bind _artselectindex (Variables|Default|GetArtSelectIndex))
  (if (== (Variables|Default|GetPaletteCenterIndex) (Variables|Default|GetArtSelectIndex))
    (bind _centerart (CallFunction|UseCenterArt))
    (return -1 _centerart)
    (else
      (return (+ _artselectindex (/ _artselectindex (Variables|Default|GetPaletteCenterIndex))) "NewEnumerator0"))))

(fn UseCenterArt
  (bind _centerartindex (Variables|Default|GetCenterArtIndex))
  (bind _centerarts (Variables|Default|GetCenterArts))
  (bind _output (Utilities|Array|Get(acopy) _centerarts _centerartindex))
  (if (Variables|Default|GetDrawWeapon)
    (if (Utilities|Enum|Equal(Enum) _output "NewEnumerator1")
      (Variables|Default|SetDrawWeapon false))
    (return _output)
    (else
      (Variables|Default|SetDrawWeapon true)
      (return "NewEnumerator3"))))