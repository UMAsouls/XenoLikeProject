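; Arts manager component that holds a character's arts and a palette with one extra slot, apparently for a central Talent Art.
; BeginPlay sizes the palette and sets the talent index to half the art count.
; SetArt writes each art to both arrays, using integer division to skip the middle slot; its range check has no Idx input.
; GetArtAbility reads abilities by palette index, while GetArtImage is an empty stub.
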(event Custom|InitArtPalette
  (bind _artdatas (Variables|Default|GetArtDatas))
  (bind _returnvalue (Utilities|Array|Length _artdatas))
  ;[0.15 0.15 0.15 0.5] アーツパレットのサイズ初期化
  (Variables|Default|SetTalentArtIdx (/ _returnvalue 2))
  (Utilities|Array|Resize (Variables|Default|GetArtPalette) (+ 1 _returnvalue)))

(event Custom|SetArtInPalette
  (params (Idx :type Integer) (Data :type Art%20Data%20Asset%20Object%20Reference))
  ;[0.15 0.15 0.15 0.5] アーツパレットにセット
  (Utilities|Array|SetArrayElem (Variables|Default|GetArtPalette) (+ Idx (/ Idx (Variables|Default|GetTalentArtIdx))) Data))

(event EventBeginPlay
  (CallFunction|InitArtPalette))

(event EventTick
  (params (DeltaSeconds :type Float%20%28single-precision%29)))

(event EventSetArt
  (params (Idx :type Integer) (Data :type Art%20Data%20Asset%20Object%20Reference))
  ;[0.15 0.15 0.15 0.5] 通常アーツセット
  (if (Math|Integer|InRange(Integer) 0 0 (Utilities|Array|Length (Variables|Default|GetArtDatas)) true false)
    (Utilities|Array|SetArrayElem (Variables|Default|GetArtDatas) Idx Data)
    (CallFunction|SetArtinPalette Idx Data)))

(fn GetArtAbility
  (params (PaletteIdx :type Integer))
  (return (Variables|/Script/XenoLikeProject.ArtDataAsset|GetArtAbility (Utilities|Array|Get(acopy) (Variables|Default|GetArtPalette) PaletteIdx))))

(fn GetArtImage
  (params (PaletteIdx :type Integer))
  (return 0))