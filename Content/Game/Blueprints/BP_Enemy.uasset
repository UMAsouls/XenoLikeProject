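; Base-style enemy character that registers with enemy-tracking subsystems, picks battle targets by hate and can be locked on to.
; BP_HateManager accumulates hate from damage and AddHate calls; lock-on switches to the top member, waiting until any active Art ability tag clears.
; Range components notify overlapping actors about lock-on availability, and a widget shows lock-on state.
; Death reports defeat, ends any chain attack, then deregisters and destroys the actor after a delay.
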(event OnComponentBeginOverlap(LockonableRange)
  (params (OverlappedComponent :type Primitive%20Component%20Object%20Reference) (OtherActor :type Actor%20Object%20Reference) (OtherComp :type Primitive%20Component%20Object%20Reference) (OtherBodyIndex :type Integer) (bFromSweep :type Boolean) (SweepResult :type Hit%20Result%20Structure%20%28by%20ref%29))
  (Class|BPIPlayer|AddinLockonRangeTarget(Message) OtherActor self))

(event OnComponentEndOverlap(LockonCountinuableRange)
  (params (OverlappedComponent :type Primitive%20Component%20Object%20Reference) (OtherActor :type Actor%20Object%20Reference) (OtherComp :type Primitive%20Component%20Object%20Reference) (OtherBodyIndex :type Integer))
  (Class|BPIPlayer|CanselLockonbyRangeOut(Message) OtherActor self))

(event OnComponentEndOverlap(LockonableRange)
  (params (OverlappedComponent :type Primitive%20Component%20Object%20Reference) (OtherActor :type Actor%20Object%20Reference) (OtherComp :type Primitive%20Component%20Object%20Reference) (OtherBodyIndex :type Integer))
  (Class|BPIPlayer|RemoveinLockonRangeTarget(Message) OtherActor self))

(event Custom|UpdateLockOnTarget
  ;[0.15 0.15 0.15 0.5] ロックオン対象メンバー更新
  (bind _member (Default|GetBestHateMember (Variables|Default|GetBP_HateManager)))
  (if (GameplayTags|HasMatchingGameplayTag (Variables|Default|GetAbilitySystem) "(TagName=\"Ability.Action.Battle.Art\")")
    (Ability|Tasks|WaitGameplayTagRemoveFromActor 0 "(TagName=\"Ability.Action.Battle.Art\")" true
      (:Removed
        _)))
  (CallFunction|LockonNewTarget _member))

(event EventBeginPlay
  (|CallParentFunction)
  (Class|CheckEnemiesExtincutionSubsystem|AddEnemy (Subsystems|GetCheckEnemiesExtincutionSubsystem) self))

(event Collision|EventActorBeginOverlap
  (params (OtherActor :type Actor%20Object%20Reference))
  (|CallParentFunction OtherActor) ; This node is disabled and will not be called.\nDrag off pins to build functionality.
)

(event EventOnLockonTargetDeath
  (Default|MemberUpdate (Variables|Default|GetBP_HateManager))
  (CallFunction|UpdateLockonTarget))

(event EventOnEquip
  (Class|EnemiesSubsystem|AddEnemy (Subsystems|GetEnemiesSubsystem) self)
  (Audio|PlaySound2D "/Game/Assets/Music/SE/maou_se_system01.maou_se_system01" 1.0 1.0 0.0 0 0))

(event EventOnUnEquip
  (Class|EnemiesSubsystem|EscapeEnemy (Subsystems|GetEnemiesSubsystem) self)
  (Default|OnBattleEnd (Variables|Default|GetBP_HateManager)))

(event EventCancelLockedon
  (params (LockOnBy :type Actor%20Object%20Reference))
  (|CallParentFunction 0)
  (Rendering|SetVisibility (Variables|Default|GetWidget) false false))

(event EventLockedon
  (params (LockOnBy :type Actor%20Object%20Reference))
  (|CallParentFunction LockOnBy)
  (Rendering|SetVisibility (Variables|Default|GetWidget) true false))

(event EventOnDeathEvent
  (Class|EnemiesSubsystem|DefeatEnemy (Subsystems|GetEnemiesSubsystem) self)
  (if (GameplayTags|HasMatchingGameplayTag (Variables|Default|GetAbilitySystem) "(TagName=\"Chara.Phase.ChainAttack\")")
    (Class|BPIXenoGameMode|ChainAttackEnd(Message) (Actor|GetComponentbyClass (Game|GetGameMode) "/Game/Game/Blueprints/Component/BP_ChainAttackManager.BP_ChainAttackManager_C")))
  (|CallParentFunction)
  (Utilities|FlowControl|Delay 3.0)
  (Class|CheckEnemiesExtincutionSubsystem|RemoveEnemy (Subsystems|GetCheckEnemiesExtincutionSubsystem) self 1)
  (Actor|DestroyActor))

(event EventOnDamageEvent
  (params (Damage :type Float%20%28single-precision%29) (SourceActor :type Actor%20Object%20Reference))
  (|CallParentFunction Damage SourceActor)
  (Default|OnDamaged (Variables|Default|GetBP_HateManager) Damage SourceActor)
  (CallFunction|UpdateLockonTarget))

(event EventTick
  (params (DeltaSeconds :type Float%20%28single-precision%29))
  (|CallParentFunction 0.0))

(event EventAddHate
  (params (Hate :type Float%20%28double-precision%29) (Source :type Actor%20Object%20Reference))
  (Default|AddHate (Variables|Default|GetBP_HateManager) Source Hate))

(fn ConstructionScript
  (|CallParentFunction))

(fn GetWasRendered
  (return (Class|PrimitiveComponent|WasRecentlyRendered (Variables|Character|GetMesh) 0.2)))