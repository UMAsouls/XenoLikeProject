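; BP_EquipedArt represents one equipped Art, pairing its data with an ability and a recast tag.
; Initialize stores all three, derives the max recast time as the inverse of the Art's recast speed, and passes the tag to the ability.
; Getters expose the Art data and tag, while CheckUseable always returns false.
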(event EventInitialize
  (params (Art :type Art%20Data%20Asset%20Object%20Reference) (Ability :type Gameplay%20Ability%20Object%20Reference) (RecastTag :type Gameplay%20Tag%20Structure))
  ;[0.15 0.15 0.15 0.5] アーツセット
  (Variables|Default|SetRecastTag RecastTag)
  (bind _output_get (Variables|Default|SetArt Art))
  (Variables|Default|SetMaxRecastTime (/ 1.0 (Variables|/Script/XenoLikeProject.ArtDataAsset|GetRecastSpeed _output_get)))
  (bind _output_get_2 (Variables|Default|SetSetAbility Ability))
  (Class|BPIArtAbility|SetRecastTag(Message) _output_get_2 (Variables|Default|GetRecastTag)))

(fn CheckUseable
  (return false))

(fn GetData
  (return (Variables|Default|GetArt)))

(fn GetRecastTag
  (return (Variables|Default|GetRecastTag)))