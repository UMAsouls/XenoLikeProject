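; Party member character for an Xenoblade-style battle system, built on GAS and driven by party, battle and enemy subsystems.
; Lock-on picks on-screen targets nearest screen center and switches left or right by screen X, wrapping around.
; An art palette with a swappable center slot fires abilities at the target; hits add hit stop, damage numbers and party gauge.
; Dead members register with overlapping allies, who spend party gauge to revive them.
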(event OnComponentBeginOverlap(CapsuleComponent)
  (params (OverlappedComponent :type Primitive%20Component%20Object%20Reference) (OtherActor :type Actor%20Object%20Reference) (OtherComp :type Primitive%20Component%20Object%20Reference) (OtherBodyIndex :type Integer) (bFromSweep :type Boolean) (SweepResult :type Hit%20Result%20Structure%20%28by%20ref%29))
  ;[0.15 0.15 0.15 0.5] 復活処理関連
  (if (Variables|Default|GetRebirthable)
    (CallFunction|AddSelftoAroundonDeath OtherActor)))

(event OnComponentEndOverlap(CapsuleComponent)
  (params (OverlappedComponent :type Primitive%20Component%20Object%20Reference) (OtherActor :type Actor%20Object%20Reference) (OtherComp :type Primitive%20Component%20Object%20Reference) (OtherBodyIndex :type Integer))
  ;[0.15 0.15 0.15 0.5] 復活処理関連
  (if (Variables|Default|GetRebirthable)
    (bind _asbp_main_character (Utilities|Casting|CastToBP_MainCharacter OtherActor))
    (Utilities|Array|RemoveItem (Variables|BP_MainCharacter_C|GetAroundDeathMemberID _asbp_main_character) (Variables|Default|GetPartyNumber))
    (Default|CallEDRebirthableActorCheck (Utilities|Array|IsNotEmpty (Variables|BP_MainCharacter_C|GetAroundDeathMemberID _asbp_main_character)))))

(event Custom|SetupInput
  ;[0.15 0.15 0.15 0.5] 入力マッピングの設定
  (Input|AddMappingContext (PlayerController|LocalPlayerSubsystems|GetEnhancedInputLocalPlayerSubsystem (Game|GetPlayerController 0)) "/Game/Game/Input/IMC_Default.IMC_Default" 0 "(bIgnoreAllPressedKeysUntilRelease=True,bForceImmediately=False,bNotifyUserSettings=False)"))

(event Custom|HitDamageDisplay
  (params (damage :type Float%20%28double-precision%29) (HitTarget :type Actor%20Object%20Reference) (widget :type User%20Widget%20Class%20Reference))
  (Utilities|IsValid HitTarget
    (:Is%20Valid
      (bind (_outhit _returnvalue) (Collision|LineTraceByChannel (Transformation|GetActorLocation) (Transformation|GetActorLocation HitTarget) "TraceTypeQuery2" false 0 "None"))
      (if _returnvalue
        (bind _returnvalue_2 (Game|SpawnActorfromClass "/Game/Game/Blueprints/Effect/BP_DamageInteger.BP_DamageInteger_C" (Math|Transform|MakeTransform (.Location (Collision|BreakHitResult _outhit))) "Undefined" "MultiplyWithRoot" 0 0))
        (Default|SetWidget _returnvalue_2 widget)
        (Class|BPIDamageInteger|SetDamage(Message) _returnvalue_2 damage)))))

(event Custom|MakeCenterArtMap
  (bind _availablearts (Variables|Default|GetavailableArts))
  (bind (_normalarts _talentart _escape _chainattack _drawweapon) (Utilities|Struct|BreakAvailableArts _availablearts))
  (Variables|Default|SetCenterArts (Utilities|Map|MakeMap "NewEnumerator0" _talentart "NewEnumerator1" _escape "NewEnumerator2" _chainattack "NewEnumerator3" _drawweapon)))

(event Custom|TimeHateReduce
  ;[0.15 0.15 0.15 0.5] 各種初期化＆バインド処理
  (CallFunction|AddAllEnemyHate (* (Variables|Const|GetReduceHate) -1.0)))

(event Custom|BindBattleSubsystemDelegate
  ;[0.15 0.15 0.15 0.5] 各種初期化＆バインド処理
  (EventDispatchers|AssignOnBattleStart (Subsystems|GetBattleSubsystem) (delegate Custom|OnBattleStart_Event))
  (EventDispatchers|AssignOnBattleEnd (Subsystems|GetBattleSubsystem) (delegate Custom|OnBattleEnd_Event)))

(event Custom|InitializeAvailableArts
  ;[0.15 0.15 0.15 0.5] 最初のavailableArts作成(仮実装)
  (CallFunction|MakeCenterArtMap)
  (CallFunction|MakeAvailableArtPos))

(event Custom|SetFirstMaxWalkSpeed
  ;[0.15 0.15 0.15 0.5] 各種初期化＆バインド処理
  (Variables|Status|SetMaxWalkSpeed (Variables|/Script/Engine.CharacterMovementComponent|GetMaxWalkSpeed (Variables|Character|GetCharacterMovement))))

(event Custom|OnBattleEnd_Event
  ;[0.15 0.15 0.15 0.5] 各種初期化＆バインド処理
  (CallFunction|UnEquip)
  (CallFunction|UnLockonTarget)
  (Utilities|Time|ClearandInvalidateTimerbyHandle (Variables|Default|GetHateReduceEventSpec)))

(event Custom|HitStop
  (Variables|/Script/Engine.Actor|SetCustomTimeDilation self 0.0)
  (Utilities|FlowControl|Delay 0.1)
  (Variables|/Script/Engine.Actor|SetCustomTimeDilation self 1.0))

(event Custom|UHP
  (params (MaxHP :type Float%20%28single-precision%29) (HP :type Float%20%28single-precision%29))
  ;[0.15 0.15 0.15 0.5] UI関連の更新
  (Default|UpdateHp (stale EventSetStatusBar StatusBar) HP MaxHP))

(event Custom|MakeAvailableArtPos
  (bind _availablearts (Variables|Default|GetavailableArts))
  (bind _normalarts (Utilities|Struct|BreakAvailableArts _availablearts))
  (bind _returnvalue (Utilities|Array|Length _normalarts))
  (bind _returnvalue_2 (/ _returnvalue 2))
  ;[0.15 0.15 0.15 0.5] ArtPalleteの有効な場所を記録
  (Variables|Default|SetNormalArtList _normalarts)
  (Utilities|Array|Resize (Variables|Default|GetArtList) (+ 1 (Utilities|Array|Length _normalarts)))
  (for (_array_element _array_index) _normalarts
    (Utilities|Array|SetArrayElem (Variables|Default|GetArtList) (+ _array_index (/ _array_index _returnvalue_2)) _array_element))
  (Variables|Default|SetCenterArtIndex _returnvalue_2)
  (CallFunction|UpdateCenterArt "NewEnumerator3"))

(event Custom|ChangeWalkSpeed
  (params (magnitude :type Float%20%28double-precision%29))
  (Variables|/Script/Engine.CharacterMovementComponent|SetMaxWalkSpeed (Variables|Character|GetCharacterMovement) (* (Variables|Status|GetMaxWalkSpeed) magnitude)))

(event Custom|AddSelfToAroundOnDeath
  (params (AroundMember :type Actor%20Object%20Reference))
  ;[0.15 0.15 0.15 0.5] 復活処理関連
  (bind _asbp_main_character (Utilities|Casting|CastToBP_MainCharacter AroundMember))
  (Utilities|Array|Add (Variables|BP_MainCharacter_C|GetAroundDeathMemberID _asbp_main_character) (Variables|Default|GetPartyNumber))
  (Default|CallEDRebirthableActorCheck _asbp_main_character (Utilities|Array|IsNotEmpty (Variables|BP_MainCharacter_C|GetAroundDeathMemberID _asbp_main_character))))

(event Custom|OnBattleStart_Event
  ;[0.15 0.15 0.15 0.5] 各種初期化＆バインド処理
  (bind _returnvalue (Utilities|Time|SetTimerbyEvent (delegate Custom|TimeHateReduce) 1.0 true true))
  (Variables|Default|SetHateReduceEventSpec _returnvalue))

(event Custom|BindAttributeSetDelegate
  ;[0.15 0.15 0.15 0.5] 各種初期化＆バインド処理
  (GameplayAttributes|GetAttributeSet (Variables|Default|GetAbilitySystem) "/Script/XenoLikeProject.XenoCharacterAttributeSet"))

(event Input|EnhancedActionEvents|EnhancedInputActionIA_Look
  (params (ActionValue :type Vector%202D%20Structure) (ElapsedSeconds :type Float%20%28double-precision%29) (TriggeredSeconds :type Float%20%28double-precision%29) (InputAction :type Input%20Action%20Object%20Reference :default "/Game/Game/Input/Actions/IA_Look.IA_Look"))
  ;[0.15 0.15 0.15 0.5] 基本アクション
  (Pawn|Input|AddControllerYawInput (.x ActionValue))
  (Pawn|Input|AddControllerPitchInput (.y ActionValue)))

(event EventBeginPlay
  ;[0.15 0.15 0.15 0.5] Beginplay
  (|CallParentFunction)
  (CallFunction|InitializeAvailableArts)
  (Class|PartySubsystem|SetPartyMember (Subsystems|GetPartySubsystem) (Variables|Default|GetPartyNumber) self)
  (GameplayAbilities|GiveAbility (Variables|Default|GetAbilitySystem) "/Game/Game/Blueprints/GamePlayAbilities/GA_Move.GA_Move_C" 0 -1)
  (CallFunction|BindAttributeSetDelegate)
  (CallFunction|BindBattleSubsystemDelegate)
  (CallFunction|SetFirstMaxWalkSpeed))

(event EventChangeNormalCamera
  (Components|Activation|Deactivate (Variables|Default|GetChainAttackCamera))
  (Components|Activation|Activate (Variables|Default|GetCamera) false))

(event EventInputJump
  ;[0.15 0.15 0.15 0.5] 基本アクション
  (Utilities|IsValid (Variables|Default|GetLockOnActor)
    (:Is%20Not%20Valid
      (Character|Jump))))

(event EventSetStatusBar
  (params (StatusBar :type WBP%20Member%20Status%20Bar%20Object%20Reference))
  (bind _abilitysystem (Variables|Default|GetAbilitySystem))
  ;[0.15 0.15 0.15 0.5] UI関連の更新
  (bind _returnvalue (GameplayAttributes|GetAttributeSet (Variables|Default|GetAbilitySystem) "/Script/XenoLikeProject.XenoCharacterAttributeSet"))
  (EventDispatchers|BindEventtoOnHPUpdate _returnvalue (delegate Custom|UHP))
  (Default|SetCharacterInfo StatusBar (Utilities|Text|ToText(Name) (Variables|Default|GetName)) (.ReturnValue (Ability|Attribute|GetFloatAttributefromAbilitySystemComponent _abilitysystem "(AttributeName=\"Hp\",Attribute=/Script/XenoLikeProject.XenoCharacterAttributeSet:Hp,AttributeOwner=\"/Script/CoreUObject.Class'/Script/XenoLikeProject.XenoCharacterAttributeSet'\")")) (.ReturnValue (Ability|Attribute|GetFloatAttributefromAbilitySystemComponent _abilitysystem "(AttributeName=\"MaxHp\",Attribute=/Script/XenoLikeProject.XenoCharacterAttributeSet:MaxHp,AttributeOwner=\"/Script/CoreUObject.Class'/Script/XenoLikeProject.XenoCharacterAttributeSet'\")")) 1 99))

(event EventLockonNewTarget
  (params (NewLockonTarget :type Actor%20Object%20Reference))
  ;[0.15 0.15 0.15 0.5] Lockon
  ;;[0.15 0.15 0.15 0.5] 新しい対象をロックオンする際の処理
  (|CallParentFunction NewLockonTarget)
  (Utilities|IsValid (Variables|Default|GetLockOnActor)
    (:Is%20Valid
      (Default|CallOnLockonTargetChanged))))

(event EventUnLockonTarget
  ;[0.15 0.15 0.15 0.5] Lockon
  (|CallParentFunction)
  (Default|CallOnUnLockonTarget))

(event EventCallMoving
  (bind _movedirection (Variables|Default|GetMoveDirection))
  (bind (_x _y) (Math|Vector2D|BreakVector2D _movedirection))
  ;[0.15 0.15 0.15 0.5] 基本アクション
  (Class|XenoLikeProjectCharacter|DoMove _x _y)
  (Variables|Default|SetMoveCalling false))

(event EventTick
  (params (DeltaSeconds :type Float%20%28single-precision%29))
  (|CallParentFunction 0.0))

(event EventUpdateCenterArt
  (params (CenterType :type CenterArtType%20Enum :default "NewEnumerator0"))
  (Variables|Default|Set%20CenterArtType CenterType)
  (Utilities|Array|SetArrayElem (Variables|Default|GetArtList) (Variables|Default|GetCenterArtIndex) (.Value (Utilities|Map|Find (Variables|Default|GetCenterArts) (Variables|Default|Get%20CenterArtType))))
  (Default|CallOnCenterArtUpdate (.Value (Utilities|Map|Find (Variables|Default|GetCenterArts) (Variables|Default|Get%20CenterArtType))) self))

(event EventUseArtbyPaletteIdx
  (params (Idx :type Integer))
  ;[0.15 0.15 0.15 0.5] アーツ使用処理
  (Utilities|IsValid (Variables|Default|GetLockOnActor)
    (:Is%20Valid
      (bind _artdata (Class|BPIEquipedArt|GetData(Message) (Utilities|Array|Get(acopy) (Variables|Default|GetArtList) Idx)))
      (CallFunction|UseArt (Variables|/Script/XenoLikeProject.ArtDataAsset|GetArtAbility _artdata)))))

(event EventOnEquip
  (CallFunction|ChangeWalkSpeed 0.75))

(event EventLockonCancel
  ;[0.15 0.15 0.15 0.5] Lockon
  (if (not (GameplayTags|HasMatchingGameplayTag (Variables|Default|GetAbilitySystem) "(TagName=\"Chara.Phase.Fight\")"))
    (if (not (Variables|/Script/XenoLikeProject.BattleSubsystem|GetIsBattle (Subsystems|GetBattleSubsystem)))
      (CallFunction|UnLockonTarget))))

(event EventAddinLockonRangeTarget
  (params (Target :type Actor%20Object%20Reference))
  ;[0.15 0.15 0.15 0.5] Lockon
  ;;[0.15 0.15 0.15 0.5] ロックオン可能範囲内ターゲット追加・削除
  (Utilities|Array|Add (Variables|Default|GetInLockonRangeTargets) Target))

(event EventOnUnEquip
  (CallFunction|ChangeWalkSpeed 1.0))

(event EventAddAllEnemyHate
  (params (Hate :type Float%20%28double-precision%29))
  ;[0.15 0.15 0.15 0.5] 各種初期化＆バインド処理
  (for _array_element (Variables|/Script/XenoLikeProject.EnemiesSubsystem|GetEnemies (Subsystems|GetEnemiesSubsystem))
    (Class|BPIEnemy|AddHate(Message) _array_element Hate self)))

(event EventRebirth
  ;[0.15 0.15 0.15 0.5] 復活処理関連
  (bind _returnvalue (Class|PartySubsystem|UsePartyGage (Subsystems|GetPartySubsystem) 1))
  (if _returnvalue
    (bind _returnvalue_2 (Ability|GameplayEffect|AssignTagSetbyCallerMagnitude (GameplayEffects|MakeOutgoingSpec :self (Variables|Default|GetAbilitySystem) :GameplayEffectClass "/Game/Game/Blueprints/GamePlayEffects/GE_HealArt.GE_HealArt_C") "(TagName=\"Effect.Heal.ArtBonus\")" 2.0))
    (GameplayEffects|ApplyGameplayEffectSpecToSelf (Variables|Default|GetAbilitySystem) _returnvalue_2)
    (Animation|Montage|PlayMontage (Variables|Character|GetMesh) "/Game/Assets/Characters/Member/Xeno3_chara_Anim_アーマチュア_001_rebirth_Montage.Xeno3_chara_Anim_アーマチュア_001_rebirth_Montage"
      (:OnBlendOut
        (Variables|Default|Set%20DeathFlag false)
        (Class|PartySubsystem|SubtractDeath (Subsystems|GetPartySubsystem) self)
        (Class|BPICharacterController|OnRebirth(Message) (Pawn|GetController))))))

(event EventOnAttackHitEvent
  (params (Damage :type Float%20%28single-precision%29) (ResultTag :type Gameplay%20Tag%20Container%20Structure) (TargetActor :type Actor%20Object%20Reference))
  ;[0.15 0.15 0.15 0.5] 各種初期化＆バインド処理
  (|CallParentFunction Damage ResultTag TargetActor)
  (CallFunction|HitStop)
  (|SwitchGameplayTagContainer ResultTag
    (:Default
      (Class|PartySubsystem|AddPartyGage (Subsystems|GetPartySubsystem) 0.03)
      (CallFunction|HitDamageDisplay Damage TargetActor "/Game/Game/Blueprints/Effect/WBP_DamageText.WBP_DamageText_C"))
    (:%28GameplayTags=%28%28TagName="Attack.Result.ExtraBonus"%29%29%29
      (Class|PartySubsystem|AddPartyGage (Subsystems|GetPartySubsystem) 0.12)
      (CallFunction|HitDamageDisplay Damage TargetActor "/Game/Game/Blueprints/Effect/WBP_ExtraDamageText.WBP_ExtraDamageText_C"))))

(event EventRebirthAroundMember
  (bind _arounddeathmemberid (Variables|Default|GetAroundDeathMemberID))
  ;[0.15 0.15 0.15 0.5] 復活処理関連
  (if (Utilities|Array|IsNotEmpty (Variables|Default|GetAroundDeathMemberID))
    (bind _returnvalue (Class|PartySubsystem|GetPartyMember (Subsystems|GetPartySubsystem) (Utilities|Array|Get(acopy) (Variables|Default|GetAroundDeathMemberID))))
    (Class|BPICharacter|Rebirth(Message) _returnvalue)
    (Utilities|Array|RemoveIndex _arounddeathmemberid)
    (Default|CallEDRebirthableActorCheck (Utilities|Array|IsNotEmpty _arounddeathmemberid))))

(event EventChangeChainAttackCamera
  (Components|Activation|Deactivate (Variables|Default|GetCamera))
  (Components|Activation|Activate (Variables|Default|GetChainAttackCamera) false))

(event EventOnLockonTargetDeath
  (bind _returnvalue (Subsystems|GetEnemiesSubsystem))
  (bind _enemies (Variables|/Script/XenoLikeProject.EnemiesSubsystem|GetEnemies _returnvalue))
  (if (Utilities|Array|IsNotEmpty _enemies)
    (CallFunction|LockonNewTarget (Utilities|Array|Get(acopy) _enemies))
    (else
      (CallFunction|UnLockonTarget))))

(event EventRemoveinLockonRangeTarget
  (params (Target :type Actor%20Object%20Reference))
  ;[0.15 0.15 0.15 0.5] Lockon
  ;;[0.15 0.15 0.15 0.5] ロックオン可能範囲内ターゲット追加・削除
  (Utilities|Array|RemoveItem (Variables|Default|GetInLockonRangeTargets) Target))

(event EventCanselLockonbyRangeout
  (params (Caller :type Actor%20Object%20Reference))
  ;[0.15 0.15 0.15 0.5] Lockon
  ;;[0.15 0.15 0.15 0.5] ロックオン継続範囲から出た場合のロックオン解除処理
  (if (== Caller (Variables|Default|GetLockOnActor))
    (CallFunction|LockonCancel)))

(event EventStopJump
  ;[0.15 0.15 0.15 0.5] 基本アクション
  (Character|StopJumping))

(event EventChangeLockon
  (params (Direction :type Float%20%28double-precision%29))
  ;[0.15 0.15 0.15 0.5] Lockon
  ;;[0.15 0.15 0.15 0.5] ロックオン対象の変更
  (Utilities|IsValid (Variables|Default|GetLockOnActor)
    (:Is%20Valid
      (bind _lockonabletargets (CallFunction|SearchLockonableTargets (Variables|Default|GetInLockonRangeTargets)))
      (bind _selectedtarget (CallFunction|SelectLockonChangeTarget _lockonabletargets (Variables|Default|GetLockOnActor) (> Direction 0.0)))
      (CallFunction|LockonNewTarget _selectedtarget))))

(event EventFirstLockon
  ;[0.15 0.15 0.15 0.5] Lockon
  ;;[0.15 0.15 0.15 0.5] 新規ロックオン
  (Utilities|IsValid (Variables|Default|GetLockOnActor)
    (:Is%20Not%20Valid
      (bind _lockonabletargets (CallFunction|SearchLockonableTargets (Variables|Default|GetInLockonRangeTargets)))
      (bind _selectedtarget (CallFunction|SelectFirstLockonTarget _lockonabletargets))
      (CallFunction|LockonNewTarget _selectedtarget)
      (Utilities|IsValid (Variables|Default|GetLockOnActor)
        (:Is%20Valid
          (Default|CallOnNewTargetLockon))))))

(event EventMove
  (params (Direction :type Vector%202D%20Structure))
  ;[0.15 0.15 0.15 0.5] 基本アクション
  (Variables|Default|SetMoveDirection Direction)
  (Variables|Default|SetMoveCalling true)
  (Abilities|TryActivateAbilitybyClass (Variables|Default|GetAbilitySystem) "/Game/Game/Blueprints/GamePlayAbilities/GA_Move.GA_Move_C" true))

(event EventOnDeathEvent
  (Class|BPICharacterController|OnDeath(Message) (Pawn|GetController))
  (Variables|Default|Set%20DeathFlag true)
  (for _array_element (Variables|Default|GetLockOnBy)
    (Class|BPICharacter|OnLockonTargetDeath(Message) _array_element))
  (Animation|Montage|PlayMontage (Variables|Character|GetMesh) (Variables|Default|GetDeathMontage)
    (:OnCompleted
      (Class|PartySubsystem|AddDeath (Subsystems|GetPartySubsystem) self)
      (for _array_element_2 (Collision|GetOverlappingActors (Variables|Default|GetRebirthableCollision) "BP_MainCharacter_C" :!class /Script/Engine.PrimitiveComponent)
        (if (not (== _array_element_2 self))
          (CallFunction|AddSelftoAroundonDeath _array_element_2)))
      (Variables|Default|SetRebirthable true))))

(fn ConstructionScript)

(fn SelectFirstLockonTarget
  (params (LockonableTargets :type Array%20of%20Actor%20Object%20References))
  (if (Utilities|Array|IsNotEmpty LockonableTargets)
    (LocalVariables|SetTempSelectedTarget (Utilities|Array|Get(acopy) LockonableTargets))
    (for _array_element LockonableTargets
      (if (< (CallFunction|GetDistancefromScreenCenter _array_element) (CallFunction|GetDistancefromScreenCenter (LocalVariables|GetTempSelectedTarget)))
        (LocalVariables|SetTempSelectedTarget _array_element)))
    (return (LocalVariables|GetTempSelectedTarget))
    (else
      (return 0))))

(fn SelectLockonChangeTarget
  (params (LockonableTargets :type Array%20of%20Actor%20Object%20References) (CurrentLockonedActor :type Actor%20Object%20Reference) (IsRight :type Boolean))
  (bind _screenlocation (CallFunction|GetScreenLocation CurrentLockonedActor))
  (if (Utilities|Array|IsNotEmpty LockonableTargets)
    (LocalVariables|SetTempSelectedTarget 0)
    (if (CallFunction|GetIsLockonable CurrentLockonedActor)
      (for _array_element LockonableTargets
        (LocalVariables|SetArrayElement _array_element)
        (if (!= (LocalVariables|GetArrayElement) CurrentLockonedActor)
          ;[0.15 0.15 0.15 0.5] 現在ロックオン対象より変えたい方向側に居るかどうかの判定
          (if (select IsRight (> (.x (.ScreenLocation (CallFunction|GetScreenLocation (LocalVariables|GetArrayElement)))) (.x _screenlocation)) (< (.x (.ScreenLocation (CallFunction|GetScreenLocation (LocalVariables|GetArrayElement)))) (.x _screenlocation)))
            ;[0.15 0.15 0.15 0.5] 現在ターゲットに最も近いアクターの判定
            (Utilities|IsValid (LocalVariables|GetTempSelectedTarget)
              (:Is%20Valid
                (if (< (CallFunction|GetScreenDistanceX CurrentLockonedActor (LocalVariables|GetArrayElement)) (CallFunction|GetScreenDistanceX (LocalVariables|GetTempSelectedTarget) CurrentLockonedActor))
                  (LocalVariables|SetTempSelectedTarget (LocalVariables|GetArrayElement))))
              (:Is%20Not%20Valid
                (LocalVariables|SetTempSelectedTarget (LocalVariables|GetArrayElement)))))))
      (Utilities|IsValid (LocalVariables|GetTempSelectedTarget)
        (:Is%20Valid
          (return (LocalVariables|GetTempSelectedTarget)))
        (:Is%20Not%20Valid
          _)))
    ;[0.15 0.15 0.15 0.5] 現ターゲット対象が画面内にないor変えたい方向に対象が居ないときの処理
    (LocalVariables|SetTempSelectedTarget (Utilities|Array|Get(acopy) LockonableTargets))
    (for _array_element_2 LockonableTargets
      (LocalVariables|SetArrayElement _array_element_2)
      ;;[0.15 0.15 0.15 0.5] 変えたい方向と逆側の端の対象の判定
      (if (select IsRight (< (.x (.ScreenLocation (CallFunction|GetScreenLocation (LocalVariables|GetArrayElement)))) (.x (.ScreenLocation (CallFunction|GetScreenLocation (LocalVariables|GetTempSelectedTarget))))) (> (.x (.ScreenLocation (CallFunction|GetScreenLocation (LocalVariables|GetArrayElement)))) (.x (.ScreenLocation (CallFunction|GetScreenLocation (LocalVariables|GetTempSelectedTarget))))))
        (LocalVariables|SetTempSelectedTarget (LocalVariables|GetArrayElement))))
    (return (LocalVariables|GetTempSelectedTarget))
    (else
      (return 0))))

(fn SearchLockonableTargets
  (params (TargetActors :type Array%20of%20Actor%20Object%20References))
  (Utilities|Array|Clear (LocalVariables|GetTempLockonAbleTargets))
  (for _array_element TargetActors
    (if (CallFunction|GetIsLockonable _array_element)
      (Utilities|Array|Add (LocalVariables|GetTempLockonAbleTargets) _array_element)))
  (return (LocalVariables|GetTempLockonAbleTargets)))

(fn GetIsLockonable
  (params (Target :type Actor%20Object%20Reference))
  (bind _returnvalue (Viewport|GetViewportSize))
  (bind (_screenlocation _success) (CallFunction|GetScreenLocation Target))
  (bind (_x _y) (Math|Vector2D|BreakVector2D _screenlocation))
  ;[0.15 0.15 0.15 0.5] カメラに映っているかどうかの判定
  (bind _wasrendered (Class|BPILockonTarget|GetWasRendered(Message) Target))
  (if _wasrendered
    (return true)
    (else
      ;[0.15 0.15 0.15 0.5] ビューポート範囲内かの判定
      (if _success
        (if (and (> (.x _returnvalue) _x) (> (.y _returnvalue) _y))
          ;[0.15 0.15 0.15 0.5] 障害物の有無の判定
          (bind _outhit (Collision|LineTraceByChannel (Transformation|GetWorldLocation (Variables|Default|GetCamera)) (Transformation|GetActorLocation Target) "TraceTypeQuery1" false (Utilities|Array|MakeArray self) "None"))
          (return (== (.HitActor (Collision|BreakHitResult _outhit)) Target))
          (else
            (return false)))
        (else
          (return false))))))

(fn GetScreenLocation
  (params (Target :type Actor%20Object%20Reference))
  (bind _returnvalue (Game|GetPlayerController 0))
  (bind _returnvalue_2 (Transformation|GetActorLocation Target))
  (bind (_screenlocation _returnvalue_3) (Class|PlayerController|ProjectWorldLocationtoScreen _returnvalue _returnvalue_2 true))
  (return _screenlocation _returnvalue_3))

(fn GetDistancefromScreenCenter
  (params (Target :type Actor%20Object%20Reference))
  (return (Math|Vector|Distance2D(Vector) (.ScreenLocation (CallFunction|GetScreenLocation Target)) (/ (Viewport|GetViewportSize) "(X=2.000000,Y=2.000000)"))))

(fn GetDistancefromScreenCenterX
  (params (Target :type Actor%20Object%20Reference))
  (return (Math|Vector|Distance2D(Vector) (Math|Vector2D|MakeVector2D (.x (.ScreenLocation (CallFunction|GetScreenLocation Target))) 0.0) (Math|Vector2D|MakeVector2D (.x (/ (Viewport|GetViewportSize) "(X=2.000000,Y=2.000000)")) 0.0))))

(fn GetScreenDistanceX
  (params (Target :type Actor%20Object%20Reference) (Target2 :type Actor%20Object%20Reference))
  (return (Math|Vector|Distance2D(Vector) (Math|Vector2D|MakeVector2D (.x (.ScreenLocation (CallFunction|GetScreenLocation Target))) 0.0) (Math|Vector2D|MakeVector2D (.x (.ScreenLocation (CallFunction|GetScreenLocation Target2))) 0.0))))

(fn GetCenterArt
  (return (Utilities|Array|Get(acopy) (Variables|Default|GetArtList) (Variables|Default|GetCenterArtIndex))))

(fn GetNormalArts
  (return (Variables|Default|GetNormalArtList)))

(fn IsAvailableArtPos
  (params (ArtIndex :type Integer))
  (return (Utilities|IsValid (Utilities|Array|Get(acopy) (Variables|Default|GetArtList) ArtIndex))))

(fn IsinAvailableArtRange
  (params (ArtIndex :type Integer))
  (return (Utilities|Array|IsValidIndex (Variables|Default|GetArtList) ArtIndex)))

(fn IsMoveCalling
  (return (and (not (GameplayTags|HasTag (GameplayTags|GetOwnedGameplayTags (Variables|Default|GetAbilitySystem) :!class /Script/GameplayTags.BlueprintGameplayTagLibrary) "(TagName=\"Chara.State.Movement.Stop\")")) (Variables|Default|GetMoveCalling))))