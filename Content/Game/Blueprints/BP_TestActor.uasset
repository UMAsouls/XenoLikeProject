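; BP_TestActor is a test actor that serves as a lock-on target and exposes an attackable collision.
; Two range components message overlapping actors to add or remove it as a candidate, or to cancel lock-on when out of range.
; Lock-on events toggle a widget, and a render query reports whether its sphere was recently drawn.
; It binds to its ability-system attribute set's damage event, but the handler is empty.
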(event OnComponentBeginOverlap(LockonableRange)
  (params (OverlappedComponent :type Primitive%20Component%20Object%20Reference) (OtherActor :type Actor%20Object%20Reference) (OtherComp :type Primitive%20Component%20Object%20Reference) (OtherBodyIndex :type Integer) (bFromSweep :type Boolean) (SweepResult :type Hit%20Result%20Structure%20%28by%20ref%29))
  (Class|BPIPlayer|AddinLockonRangeTarget(Message) OtherActor self))

(event OnComponentEndOverlap(LockonableRange)
  (params (OverlappedComponent :type Primitive%20Component%20Object%20Reference) (OtherActor :type Actor%20Object%20Reference) (OtherComp :type Primitive%20Component%20Object%20Reference) (OtherBodyIndex :type Integer))
  (Class|BPIPlayer|RemoveinLockonRangeTarget(Message) OtherActor self))

(event OnComponentEndOverlap(LockonCountinuableRange)
  (params (OverlappedComponent :type Primitive%20Component%20Object%20Reference) (OtherActor :type Actor%20Object%20Reference) (OtherComp :type Primitive%20Component%20Object%20Reference) (OtherBodyIndex :type Integer))
  (Class|BPIPlayer|CanselLockonbyRangeOut(Message) OtherActor self))

(event Custom|OnDamage
  (params (Damage :type Float%20%28single-precision%29)))

(event EventBeginPlay
  (bind _returnvalue (GameplayAttributes|GetAttributeSet (Variables|Default|GetAbilitySystem) "/Script/XenoLikeProject.XenoCharacterAttributeSet"))
  (EventDispatchers|BindEventtoOnDamage _returnvalue (delegate Custom|OnDamage)))

(event EventCancelLockedon
  (Rendering|SetVisibility (Variables|Default|GetWidget) false false))

(event EventLockedon
  (params (LockOnBy :type Actor%20Object%20Reference))
  (Rendering|SetVisibility (Variables|Default|GetWidget) true false))

(fn ConstructionScript)

(fn GetAttackableCollision
  (return (Variables|Default|GetCapsuleComponent)))

(fn GetWasRendered
  (return (Class|PrimitiveComponent|WasRecentlyRendered (Variables|Default|GetSphere1) 0.2)))