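; Base battle character for a Xenoblade-style combat system on GAS, with auto-attacks, arts, lock-on and weapon draw/sheathe.
; BeginPlay grants abilities, builds equipped-art objects from data and binds attribute-set combat events; auto-attack hits charge the talent recast.
; Tick applies relative-position effects from a dot product against the lock-on target, while an overlap volume tracks auto-attack range.
; Art readiness derives from cooldown effects or talent attributes.
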(event OnComponentBeginOverlap(AutoAttackRangeCollision)
  (params (OverlappedComponent :type Primitive%20Component%20Object%20Reference) (OtherActor :type Actor%20Object%20Reference) (OtherComp :type Primitive%20Component%20Object%20Reference) (OtherBodyIndex :type Integer) (bFromSweep :type Boolean) (SweepResult :type Hit%20Result%20Structure%20%28by%20ref%29))
  ;[0.15 0.15 0.15 0.5] AutoAttackRangeに入ってるかの判定
  (bind _collision (Class|BPILockonTarget|GetAttackableCollision(Message) OtherActor))
  (if (== _collision OtherComp)
    (if (== OtherActor (Variables|Default|GetLockOnActor))
      (Variables|Default|SetIs%20in%20Auto%20Attack%20Range true))))

(event OnComponentEndOverlap(AutoAttackRangeCollision)
  (params (OverlappedComponent :type Primitive%20Component%20Object%20Reference) (OtherActor :type Actor%20Object%20Reference) (OtherComp :type Primitive%20Component%20Object%20Reference) (OtherBodyIndex :type Integer))
  ;[0.15 0.15 0.15 0.5] AutoAttackRangeに入ってるかの判定
  (bind _collision (Class|BPILockonTarget|GetAttackableCollision(Message) OtherActor))
  (if (== _collision OtherComp)
    (if (== (Variables|Default|GetLockOnActor) OtherActor)
      (Variables|Default|SetIs%20in%20Auto%20Attack%20Range false))))

(event Custom|ApplyData
  (bind _returnvalue (GameplayAttributes|GetAttributeSet (Variables|Default|GetAbilitySystem) "/Script/XenoLikeProject.XenoCharacterAttributeSet"))
  (Class|XenoCharacterAttributeSet|SetStatus _returnvalue (Variables|Default|GetFirstStatus))
  (Variables|Default|SetavailableArts (CallFunction|MakeAvailableArts (Variables|Default|GetNormalArts) (Variables|Default|GetTalentArt) "/Game/Assets/UnEquipData.UnEquipData" "/Game/Assets/ChainAttack.ChainAttack" "/Game/Assets/EquipData.EquipData")))

(event Custom|HitDamageDisplay
  (params (damage :type Float%20%28double-precision%29) (HitTarget :type Actor%20Object%20Reference) (widget :type User%20Widget%20Class%20Reference))
  (bind (_hit _location) (CallFunction|CalculateDamageDisplayLocation HitTarget))
  (Development|PrintString (Utilities|String|ToString(Boolean) _hit))
  (if _hit
    (bind _returnvalue (Game|SpawnActorfromClass "/Game/Game/Blueprints/Effect/BP_DamageInteger.BP_DamageInteger_C" (Math|Transform|MakeTransform _location) "Undefined" "MultiplyWithRoot" 0 0))
    (Default|SetWidget _returnvalue widget)
    (Class|BPIDamageInteger|SetDamage(Message) _returnvalue damage)))

(event Custom|CalculateTargetLocalPosition
  (bind _lockonactor (Variables|Default|GetLockOnActor))
  (GameplayEffects|RemoveActiveEffectswithGrantedTags (Variables|Default|GetAbilitySystem) "(GameplayTags=((TagName=\"Chara.Target.Back\"),(TagName=\"Chara.Target.Forward\"),(TagName=\"Chara.Target.Side\")))")
  (Utilities|IsValid _lockonactor
    (:Is%20Valid
      (GameplayEffects|ApplyGameplayEffectToSelf :self (Variables|Default|GetAbilitySystem) :GameplayEffectClass (Utilities|Array|Get(acopy) (Variables|Default|GetPlaceEffects) (+ (Math|Float|Truncate (/ (Math|Vector|DotProduct (Math|Vector|Normalize (- (Transformation|GetActorLocation _lockonactor) (Transformation|GetActorLocation))) (Transformation|GetActorForwardVector (Variables|Default|GetLockOnActor))) (Math|Trig|Cos(Degrees) 45.0))) 1))))))

(event Custom|LookAtLockOnTargetNow
  (Transformation|SetActorRotation (Math|Rotator|FindLookatRotation (Transformation|GetActorLocation) (Transformation|GetActorLocation (Variables|Default|GetLockOnActor)))))

(event Custom|OnHeal_Event
  (params (Heal :type Float%20%28single-precision%29))
  (bind _returnvalue (Game|SpawnActorfromClass "/Game/Game/Blueprints/Effect/BP_DamageInteger.BP_DamageInteger_C" (Transformation|GetActorTransform) "Undefined" "MultiplyWithRoot" 0 0))
  (Default|SetWidget _returnvalue "/Game/Game/Blueprints/Effect/WBP_HealText.WBP_HealText_C")
  (Class|BPIDamageInteger|SetDamage(Message) _returnvalue Heal))

(event Custom|OnDamage_Event
  (params (Damage :type Float%20%28single-precision%29) (SourceActor :type Actor%20Object%20Reference))
  (Class|BPICharacterController|Damaged(Message) (Pawn|GetController) Damage))

(event Custom|OnAttackHit_Event
  (params (Damage :type Float%20%28single-precision%29) (ResultTag :type Gameplay%20Tag%20Container%20Structure) (TargetActor :type Actor%20Object%20Reference))
  (|SwitchGameplayTagContainer ResultTag
    (:%28GameplayTags=%28%28TagName="Attack.Kind.AutoAttack"%29%29%29
      (CallFunction|OnAutoAttackHit))))

(event Custom|OnDeath_Event
  (Class|BPICharacterController|OnDeath(Message) (Pawn|GetController))
  (Variables|Default|Set%20DeathFlag true)
  (Abilities|TryActivateAbilitybyClass (Variables|Default|GetAbilitySystem) "/Game/Game/Blueprints/GamePlayAbilities/GA_ArtStop.GA_ArtStop_C" true)
  (for _array_element (Variables|Default|GetLockOnBy)
    (Class|BPICharacter|OnLockonTargetDeath(Message) _array_element))
  (Animation|Montage|PlayMontage (Variables|Character|GetMesh) (Variables|Animation|GetDeathMontage)))

(event Custom|BindOnFightPhaseTagChanged
  (GameplayTags|BindEventWrappertoGameplayTagChanged (Variables|Default|GetAbilitySystem) "(TagName=\"Chara.Phase.Fight\")" (delegate Custom|OnFightPhaseTagChanged)))

(event Custom|OnFightPhaseTagChanged
  (params (Tag :type Gameplay%20Tag%20Structure%20%28by%20ref%29) (TagCount :type Integer))
  (bind _returnvalue (> TagCount 0))
  (Default|CallEDonFightPhaseTagChanged _returnvalue)
  (if _returnvalue
    (CallFunction|OnEquip)
    (else
      (CallFunction|OnUnEquip))))

(event Custom|OnAutoAttackHit
  (bind _returnvalue (Ability|GameplayEffect|AssignTagSetbyCallerMagnitude (GameplayEffects|MakeOutgoingSpec :self (Variables|Default|GetAbilitySystem) :GameplayEffectClass "/Game/Game/Blueprints/GamePlayEffects/GE_TalentArtRecast_Add.GE_TalentArtRecast_Add_C") "(TagName=\"Data.Cooldown.Talent\")" 1.0))
  (GameplayEffects|ApplyGameplayEffectSpecToSelf (Variables|Default|GetAbilitySystem) _returnvalue))

(event Custom|OnAttackMissed_Event
  (params (ResultTag :type Gameplay%20Tag%20Container%20Structure)))

(event Custom|OnEquip)

(event Custom|OnUnEquip)

(event EventBeginPlay
  (GameplayAbilities|GiveAbility (Variables|Default|GetAbilitySystem) (Variables|Default|GetAutoAttackAbility) 0 -1)
  (GameplayAbilities|GiveAbility (Variables|Default|GetAbilitySystem) "/Game/Game/Blueprints/GamePlayAbilities/GA_Equip.GA_Equip_C" 0 -1)
  (GameplayAbilities|GiveAbility (Variables|Default|GetAbilitySystem) "/Game/Game/Blueprints/GamePlayAbilities/GA_UnEquip.GA_UnEquip_C" 0 -1)
  (GameplayAbilities|GiveAbility (Variables|Default|GetAbilitySystem) "/Game/Game/Blueprints/GamePlayAbilities/GA_TalentArtRecast.GA_TalentArtRecast_C" 0 -1)
  (GameplayAbilities|GiveAbility (Variables|Default|GetAbilitySystem) "/Game/Game/Blueprints/GamePlayAbilities/GA_ArtStop.GA_ArtStop_C" 0 -1)
  (CallFunction|ApplyData)
  (CallFunction|BindonFightPhaseTagChanged)
  (bind _returnvalue (GameplayAttributes|GetAttributeSet (Variables|Default|GetAbilitySystem) "/Script/XenoLikeProject.XenoCharacterAttributeSet"))
  (Utilities|FlowControl|Sequence
    (:then_0
      (EventDispatchers|BindEventtoOnDamage _returnvalue (delegate Custom|OnDamage_Event))
      (EventDispatchers|BindEventtoOnDeath _returnvalue (delegate Custom|OnDeath_Event)))
    (:then_1
      (EventDispatchers|AssignOnAttackHit _returnvalue (delegate Custom|OnAttackHit_Event))
      (EventDispatchers|AssignOnAttackMissed _returnvalue (delegate Custom|OnAttackMissed_Event))
      (EventDispatchers|AssignOnHeal _returnvalue (delegate Custom|OnHeal_Event)))))

(event EventOnLockonTargetDeath)

(event EventChangeChainAttackMode
  (params (active :type Boolean))
  (if active
    (if (GameplayTags|HasMatchingGameplayTag (Variables|Default|GetAbilitySystem) "(TagName=\"Ability.Action.Battle.Art\")")
      (Ability|Tasks|WaitGameplayTagRemoveFromActor 0 "(TagName=\"Ability.Action.Battle.Art\")" true
        (:then
          (GameplayEffects|RemoveActiveEffectswithGrantedTags (Variables|Default|GetAbilitySystem) "(GameplayTags=((TagName=\"Art.Cooldown.Art1\"),(TagName=\"Art.Cooldown.Art2\"),(TagName=\"Art.Cooldown.Art3\"),(TagName=\"Art.Cooldown.Art4\")))"))
        (:Removed
          (GameplayEffects|ApplyGameplayEffectToSelf :self (Variables|Default|GetAbilitySystem) :GameplayEffectClass "/Game/Game/Blueprints/GamePlayEffects/GE_ChainAttack.GE_ChainAttack_C" :!label _label)))
      (else
        (goto _label)))
    (else
      (GameplayEffects|RemoveActiveEffectswithGrantedTags (Variables|Default|GetAbilitySystem) "(GameplayTags=((TagName=\"Chara.Phase.ChainAttack\")))"))))

(event EventCancelLockedon
  (params (LockOnBy :type Actor%20Object%20Reference))
  (Utilities|Array|RemoveItem (Variables|Default|GetLockOnBy) LockOnBy))

(event EventLockedon
  (params (LockOnBy :type Actor%20Object%20Reference))
  (Utilities|Array|Add (Variables|Default|GetLockOnBy) LockOnBy))

(event EventTick
  (params (DeltaSeconds :type Float%20%28single-precision%29))
  (CallFunction|CalculateTargetLocalPosition)
  (Utilities|IsValid (Variables|Default|GetLockOnActor)
    (:Is%20Valid
      (if (Variables|Default|GetSetPendingLookAt)
        (Transformation|SetActorRotation (Math|Rotator|FindLookatRotation (Transformation|GetActorLocation) (Transformation|GetActorLocation (Variables|Default|GetLockOnActor))))
        (Variables|Default|SetSetPendingLookAt false)))))

(event EventEquip
  (Abilities|TryActivateAbilitybyClass (Variables|Default|GetAbilitySystem) "/Game/Game/Blueprints/GamePlayAbilities/GA_Equip.GA_Equip_C" true))

(event EventLockonNewTarget
  (params (NewLockonTarget :type Actor%20Object%20Reference))
  ;[0.15 0.15 0.15 0.5] 新しい対象をロックオンする際の処理
  (Class|BPILockonTarget|CancelLockedon(Message) (Variables|Default|GetLockOnActor) self)
  (bind _result (Class|BPICharacter|GetIsDeath(Message) NewLockonTarget))
  (if (not _result)
    (bind _output_get (Variables|Default|SetLockOnActor NewLockonTarget))
    (Utilities|IsValid (Variables|Default|GetLockOnActor)
      (:Is%20Valid
        (Class|BPILockonTarget|Lockedon(Message) _output_get self)
        (bind _attack_able (CallFunction|IsAutoAttackAble (Variables|Default|GetLockOnActor)))
        (Variables|Default|SetIs%20in%20Auto%20Attack%20Range _attack_able))
      (:Is%20Not%20Valid
        (CallFunction|UnLockonTarget)))))

(event EventUseArt
  (params (Ability :type Gameplay%20Ability%20Class%20Reference))
  (if (or (== Ability "/Game/Game/Blueprints/GamePlayAbilities/GA_Equip.GA_Equip_C") (GameplayTags|HasMatchingGameplayTag (Variables|Default|GetAbilitySystem) "(TagName=\"Chara.Phase.Fight\")"))
    _
    (else
      (CallFunction|Equip)))
  (Abilities|TryActivateAbilitybyClass (Variables|Default|GetAbilitySystem) Ability true))

(event EventUnEquip
  (Abilities|TryActivateAbilitybyClass (Variables|Default|GetAbilitySystem) "/Game/Game/Blueprints/GamePlayAbilities/GA_UnEquip.GA_UnEquip_C" true))

(event EventLookatLockonTarget
  (Variables|Default|SetSetPendingLookAt true))

(event EventUnLockonTarget
  (Utilities|IsValid (Variables|Default|GetLockOnActor)
    (:Is%20Valid
      (Class|BPILockonTarget|CancelLockedon(Message) (Variables|Default|GetLockOnActor) self)
      (Variables|Default|SetLockOnActor 0))))

(event EventAutoAttack
  (Abilities|TryActivateAbilitiesbyTag (Variables|Default|GetAbilitySystem) (GameplayTags|MakeLiteralGameplayTagContainer "(GameplayTags=((TagName=\"Ability.Action.Battle.AutoAttack\")))") false))

(fn ConstructionScript)

(fn IsAutoAttackAble
  (params (Target :type Actor%20Object%20Reference))
  (bind _collision (Class|BPILockonTarget|GetAttackableCollision(Message) Target))
  (return (Class|PrimitiveComponent|IsOverlappingComponent (Variables|Default|GetAutoAttackRangeCollision) _collision)))

(fn GetSelectComponent
  (return 0))

(fn MakeEquipedArt
  (params (ArtData :type Art%20Data%20Asset%20Object%20Reference) (RecastTag :type Gameplay%20Tag%20Structure))
  (bind _returnvalue (GameplayAbilities|GiveAbility (Variables|Default|GetAbilitySystem) (Variables|/Script/XenoLikeProject.ArtDataAsset|GetArtAbility ArtData) 0 -1))
  (bind _returnvalue_2 (Game|ConstructObjectfromClass "/Game/Game/Blueprints/BP_EquipedArt.BP_EquipedArt_C"))
  (Class|BPIEquipedArt|Initialize(Message) _returnvalue_2 ArtData (.ReturnValue (Ability|GameplayAbility|GetGameplayAbilityfromSpecHandle (Variables|Default|GetAbilitySystem) _returnvalue)) RecastTag)
  (return _returnvalue_2))

(fn MakeAvailableArts
  (params (NormalArts :type Array%20of%20Art%20Data%20Asset%20Object%20References) (TalentArt :type Art%20Data%20Asset%20Object%20Reference) (Escape :type Art%20Data%20Asset%20Object%20Reference) (ChainAttack :type Art%20Data%20Asset%20Object%20Reference) (DrawWeapon :type Art%20Data%20Asset%20Object%20Reference))
  (return (Utilities|Struct|MakeAvailableArts (CallFunction|MakeNormalEquipedArts NormalArts) (CallFunction|MakeEquipedArt TalentArt "(TagName=\"Art.Cooldown.Talent\")") (CallFunction|MakeEquipedArt Escape "(TagName=\"Art.Cooldown.NoRecast\")") (CallFunction|MakeEquipedArt ChainAttack "(TagName=\"Art.Cooldown.NoRecast\")") (CallFunction|MakeEquipedArt DrawWeapon "(TagName=\"Art.Cooldown.NoRecast\")"))))

(fn SetNormalArt
  (params (Idx :type Integer) (NewArtData :type Art%20Data%20Asset%20Object%20Reference)))

(fn MakeNormalEquipedArts
  (params (Arts :type Array%20of%20Art%20Data%20Asset%20Object%20References))
  (bind _normalequipedarts (CallFunction|MakeNormalEquipedArtsRecrusion Arts))
  (return _normalequipedarts))

(fn MakeNormalEquipedArtsRecrusion
  (params (Arts :type Array%20of%20Art%20Data%20Asset%20Object%20References) (Index :type Integer) (SetArray :type Array%20of%20Object%20Object%20References))
  (LocalVariables|SetLocalArts Arts)
  (LocalVariables|SetLocalIndex Index)
  (LocalVariables|SetLocalSettingArray SetArray)
  (if (Utilities|Array|IsValidIndex (LocalVariables|GetLocalArts) (LocalVariables|GetLocalIndex))
    (Utilities|Array|SetArrayElem (LocalVariables|GetLocalSettingArray) (LocalVariables|GetLocalIndex) (CallFunction|MakeEquipedArt (Utilities|Array|Get(acopy) (LocalVariables|GetLocalArts) (LocalVariables|GetLocalIndex)) (Utilities|Array|Get(acopy) (LocalVariables|GetRecastTags) (LocalVariables|GetLocalIndex))) true)
    (bind _normalequipedarts (CallFunction|MakeNormalEquipedArtsRecrusion (LocalVariables|GetLocalArts) (+ (LocalVariables|GetLocalIndex) 1) (LocalVariables|GetLocalSettingArray)))
    (return _normalequipedarts)
    (else
      (return (LocalVariables|GetLocalSettingArray)))))

(fn IsDeath
  (return (Variables|Default|Get%20DeathFlag)))

(fn CalculateDamageDisplayLocation
  (params (Target :type Actor%20Object%20Reference))
  (Utilities|IsValid Target
    (:Is%20Valid
      (bind (_outhit _returnvalue) (Collision|LineTraceByChannel (Transformation|GetActorLocation) (Transformation|GetActorLocation Target) "TraceTypeQuery2" false 0 "None"))
      (return _returnvalue (.Location (Collision|BreakHitResult _outhit))))
    (:Is%20Not%20Valid
      (return false "0, 0, 0"))))

(fn AutoAttackAble
  (return (and (Variables|Default|GetIs%20in%20Auto%20Attack%20Range) (Utilities|IsValid (Variables|Default|GetLockOnActor)))))

(fn GetAttackableCollision
  (return (Variables|Default|GetCapsuleComponent)))

(fn GetAutoAttackCooldownTime
  (return (.ReturnValue (Ability|Attribute|GetFloatAttributefromAbilitySystemComponent (Variables|Default|GetAbilitySystem) "(AttributeName=\"AutoAttackCooldownTime\",Attribute=/Script/XenoLikeProject.XenoCharacterAttributeSet:AutoAttackCooldownTime,AttributeOwner=\"/Script/CoreUObject.Class'/Script/XenoLikeProject.XenoCharacterAttributeSet'\")"))))

(fn GetAutoAttackSpeed
  (return (.ReturnValue (Ability|Attribute|GetFloatAttributefromAbilitySystemComponent (Variables|Default|GetAbilitySystem) "(AttributeName=\"AutoAttackSpeed\",Attribute=/Script/XenoLikeProject.XenoCharacterAttributeSet:AutoAttackSpeed,AttributeOwner=\"/Script/CoreUObject.Class'/Script/XenoLikeProject.XenoCharacterAttributeSet'\")"))))

(fn GetCharacterType
  (return (Variables|Default|GetCharacterType)))

(fn GetCurrentArtRecast
  (params (RecastTag :type Gameplay%20Tag%20Structure))
  (bind _self self)
  (if (GameplayTags|MatchesTag RecastTag "(TagName=\"Art.Cooldown.Talent\")" true)
    (return (- 1.0 (/ (.ReturnValue (Ability|Attribute|GetFloatAttribute _self "(AttributeName=\"TalentArtGage\",Attribute=/Script/XenoLikeProject.XenoCharacterAttributeSet:TalentArtGage,AttributeOwner=\"/Script/CoreUObject.Class'/Script/XenoLikeProject.XenoCharacterAttributeSet'\")")) (.ReturnValue (Ability|Attribute|GetFloatAttribute _self "(AttributeName=\"TalentArtGageMax\",Attribute=/Script/XenoLikeProject.XenoCharacterAttributeSet:TalentArtGageMax,AttributeOwner=\"/Script/CoreUObject.Class'/Script/XenoLikeProject.XenoCharacterAttributeSet'\")")))))
    (else
      (bind _returnvalue (Class|AbilitySystemComponent|GetActiveEffects (Variables|Default|GetAbilitySystem) (Utilities|Struct|MakeGameplayEffectQuery "(null).None" (GameplayTags|MakeGameplayTagQueryMatchAnyTags (GameplayTags|MakeGameplayTagContainerfromTag RecastTag)))))
      (if (Utilities|Array|IsNotEmpty _returnvalue)
        (Utilities|FlowControl|Sequence
          (:then_0
            (bind _returnvalue_2 (Ability|GameplayEffect|GetActiveGameplayEffectRemainingDuration (Utilities|Array|Get(acopy) _returnvalue))))
          (:then_1
            (bind _returnvalue_3 (Class|AbilitySystemBlueprintLibrary|GetActiveGameplayEffectTotalDuration (Utilities|Array|Get(acopy) _returnvalue)))
            (return (/ _returnvalue_2 _returnvalue_3))))
        (else
          (return 0.0))))))

(fn GetCurrentLockonTarget
  (return (Variables|Default|GetLockOnActor)))

(fn GetIsDeath
  (bind _returnvalue (CallFunction|IsDeath))
  (return _returnvalue))

(fn GetName
  (return (Variables|Default|GetName)))

(fn GetUsableNormalArtSlot
  (for _array_element (.NormalArts (Utilities|Struct|BreakAvailableArts (Variables|Default|GetavailableArts)))
    (bind _recasttag (Class|BPIEquipedArt|GetRecastTag(Message) _array_element))
    (bind _recast (CallFunction|GetCurrentArtRecast _recasttag))
    (if (<= _recast 0.0)
      (Utilities|Array|Add (LocalVariables|GetUsableArts) _array_element)))
  (return (LocalVariables|GetUsableArts)))

(fn GetUsableTalentArtSlot
  (bind _availablearts (Variables|Default|GetavailableArts))
  (bind _talentart (Utilities|Struct|BreakAvailableArts _availablearts))
  (bind _recasttag (Class|BPIEquipedArt|GetRecastTag(Message) _talentart))
  (bind _recast (CallFunction|GetCurrentArtRecast _recasttag))
  (if (<= _recast 0.0)
    (return _talentart)
    (else
      (return 0))))

(fn GetWasRendered
  (return (Class|PrimitiveComponent|WasRecentlyRendered (Variables|Character|GetMesh) 0.1)))

(fn IsNormalArtUseable
  (bind _artslots (CallFunction|GetUsableNormalArtSlot))
  (return (Utilities|Array|IsNotEmpty _artslots)))

(fn IsTalentArtUseable
  (bind _artslot (CallFunction|GetUsableTalentArtSlot))
  (return (Utilities|IsValid _artslot)))