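; Art select component that manages a battle palette of arts and the selection cursor, and uses the selected art.
; Initialization recursively fills normal arts around a center slot, which holds Talent Art, Escape, Chain Attack or Draw Weapon.
; Selection recursively skips empty slots; center cycling is locked on Draw Weapon, which UnEquip sets and Equip replaces with Talent Art.
; Selection and center changes are broadcast through event dispatcher calls.
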(event Custom|SetAvailableArts
  ;[0.15 0.15 0.15 0.5] アーツパレットの初期化
  (Variables|Default|SetCenterArts (Utilities|Map|MakeMap "NewEnumerator0" (Variables|Default|GetTalentArt) "NewEnumerator1" (Variables|Default|GetEscape) "NewEnumerator2" (Variables|Default|GetChainAttack) "NewEnumerator3" (Variables|Default|GetDraw%20Weapon)))
  (CallFunction|SetNormalArts)
  (CallFunction|UpdateCenterArt))

(event Custom|UpdateCenterArt
  ;[0.15 0.15 0.15 0.5] 中央のアーツを更新
  (Utilities|Array|SetArrayElem (Variables|Default|GetArtPalette) (Variables|Default|GetPaletteCenterIndex) (.Value (Utilities|Map|Find (Variables|Default|GetCenterArts) (Variables|Default|GetCenterArtType))))
  (Default|CallEDonCenterArtChanged (CallFunction|GetCenterArt)))

(event EventBeginPlay)

(event EventTick
  (params (DeltaSeconds :type Float%20%28single-precision%29)))

(event EventSelectArt
  (params (Direction :type Float%20%28double-precision%29))
  ;[0.15 0.15 0.15 0.5] アーツ選択処理
  (bind _artsetindex (CallFunction|SearchArtsSetIndex (Math|Float|Truncate Direction) (Variables|Default|GetArtSelectIndex)))
  (if (!= _artsetindex -1)
    (bind _output_get (Variables|Default|SetArtSelectIndex _artsetindex))
    (Default|CallEDonSelectArt _output_get)))

(event EventInitialize
  (params (Data :type Available%20Arts%20Structure))
  (bind _artpalette (Variables|Default|GetArtPalette))
  ;[0.15 0.15 0.15 0.5] Index初期化
  (|CallParentFunction Data)
  (Variables|Default|SetArtSelectIndex (Variables|Default|GetPaletteCenterIndex))
  (Utilities|Array|Clear _artpalette)
  (Utilities|Array|Resize _artpalette (Variables|Default|GetPaletteLength))
  (CallFunction|SetAvailableArts))

(event EventEquip
  (Variables|Default|SetCenterArtType "NewEnumerator0")
  (CallFunction|UpdateCenterArt))

(event EventUnEquip
  (Variables|Default|SetCenterArtType "NewEnumerator3")
  (CallFunction|UpdateCenterArt))

(event EventSelectCenterArt
  (params (Direction :type Float%20%28double-precision%29))
  ;[0.15 0.15 0.15 0.5] 中央のアイコン変更
  (if (Utilities|Enum|NotEqual(Enum) (Variables|Default|GetCenterArtType) "NewEnumerator3")
    (if (Utilities|Array|IsValidIndex (Variables|Default|GetBattleCenterArtTypes) (+ (Math|Float|Truncate Direction) (Variables|Default|GetCenterArtIndex)))
      (bind _output_get (Variables|Default|SetCenterArtIndex (+ (Math|Float|Truncate Direction) (Variables|Default|GetCenterArtIndex))))
      (Variables|Default|SetCenterArtType (Utilities|Array|Get(acopy) (Variables|Default|GetBattleCenterArtTypes) _output_get))
      (CallFunction|UpdateCenterArt))))

(fn GetSelectingArt
  (return (Utilities|Array|Get(acopy) (Variables|Default|GetArtPalette) (Variables|Default|GetArtSelectIndex))))

(fn SearchArtsSetIndex
  (params (Direction :type Integer) (StartIndex :type Integer))
  (bind _output_get (LocalVariables|Setdir Direction))
  (LocalVariables|SetNextIndex (+ _output_get StartIndex))
  (if (Utilities|Array|IsValidIndex (Variables|Default|GetArtPalette) (LocalVariables|GetNextIndex))
    (Utilities|IsValid (Utilities|Array|Get(acopy) (Variables|Default|GetArtPalette) (LocalVariables|GetNextIndex))
      (:Is%20Valid
        (return (LocalVariables|GetNextIndex)))
      (:Is%20Not%20Valid
        (bind _artsetindex (CallFunction|SearchArtsSetIndex (LocalVariables|Getdir) (LocalVariables|GetNextIndex)))
        (return _artsetindex)))
    (else
      (return -1))))

(fn SetNormalArts
  (params (CurrentIndex :type Integer))
  (bind _output_get (LocalVariables|SetIndex CurrentIndex))
  (LocalVariables|SetPaletteIndex (+ _output_get (/ CurrentIndex (Variables|Default|GetPaletteCenterIndex))))
  (if (Utilities|Array|IsValidIndex (Variables|Default|GetArtPalette) (LocalVariables|GetPaletteIndex))
    (Utilities|Array|SetArrayElem (Variables|Default|GetArtPalette) (LocalVariables|GetPaletteIndex) (Utilities|Array|Get(acopy) (Variables|Default|GetNormalArts) (LocalVariables|GetIndex)))
    (bind _result (Math|Integer|IncrementInt (LocalVariables|GetIndex))
      (:%20%20
        (CallFunction|SetNormalArts _result)))))

(fn GetCenterArt
  (return (Utilities|Array|Get(acopy) (Variables|Default|GetArtPalette) (Variables|Default|GetPaletteCenterIndex))))

(fn UseSelectingArt
  (bind _ability (CallFunction|UseArt (Utilities|Array|Get(acopy) (Variables|Default|GetArtPalette) (Variables|Default|GetArtSelectIndex))))
  (return _ability))