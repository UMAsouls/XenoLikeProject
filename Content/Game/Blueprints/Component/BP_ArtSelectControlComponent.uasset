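; Main character component that tracks battle Art selection: the selected palette slot and the center Art.
; Slot selection searches recursively in the input direction, skipping unavailable positions and stopping at the range edge, using character message queries.
; Center Art cycles with wraparound through a type list unless in the unequipped type, and each change is pushed to the character.
; Initialization, palette creation and lock-off reset the slot; equip and unequip set the center type.
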(event Custom|Initialize
  (params (MainCharacter :type Actor%20Object%20Reference))
  (Variables|Default|SetMainCharacter MainCharacter)
  (bind _output_get (Variables|Default|SetArtSelectIndex 2))
  (Default|CallEDonSelectArt _output_get)
  (Variables|Default|SetCenterArtIndex 1)
  (CallFunction|CenterArtUpdate "NewEnumerator0"))

(event Custom|CenterArtUpdate
  (params (CenterArt :type CenterArtType%20Enum :default "NewEnumerator0"))
  (Class|BPIControlCharacter|UpdateCenterArt(Message) (Variables|Default|GetMainCharacter) CenterArt))

(event Custom|OnUnLockOn
  (bind _output_get (Variables|Default|SetArtSelectIndex 2))
  (Default|CallEDonSelectArt _output_get)
  (Variables|Default|SetCenterArtIndex 1))

(event Custom|CreatePalette
  (bind _output_get (Variables|Default|SetArtSelectIndex 2))
  (Default|CallEDonSelectArt _output_get))

(event EventBeginPlay)

(event EventTick
  (params (DeltaSeconds :type Float%20%28single-precision%29)))

(event EventSelectCenterArt
  (params (Direction :type Float%20%28double-precision%29))
  (if (Utilities|Enum|NotEqual(Enum) (Variables|Default|GetCenterArtType) "NewEnumerator3")
    (bind _output_get (Variables|Default|SetCenterArtIndex (Class|KismetMathLibrary|Wrap (+ (Math|Float|Truncate Direction) (Variables|Default|GetCenterArtIndex)) 0 (Utilities|Array|Length (Variables|Default|GetBattleCenterArtTypes)))))
    (bind _output_get_2 (Variables|Default|SetCenterArtType (Utilities|Array|Get(acopy) (Variables|Default|GetBattleCenterArtTypes) _output_get)))
    (CallFunction|CenterArtUpdate _output_get_2)))

(event EventSelectArt
  (params (Direction :type Float%20%28double-precision%29))
  (bind _artsetindex (CallFunction|SearchArtSetIndex (Math|Float|Truncate Direction) (Variables|Default|GetArtSelectIndex)))
  (if (!= _artsetindex -1)
    (bind _output_get (Variables|Default|SetArtSelectIndex _artsetindex))
    (Default|CallEDonSelectArt _output_get)))

(event EventEquip
  (bind _output_get (Variables|Default|SetCenterArtType "NewEnumerator0"))
  (Variables|Default|SetCenterArtIndex 1)
  (CallFunction|CenterArtUpdate _output_get))

(event EventUnEquip
  (bind _output_get (Variables|Default|SetCenterArtType "NewEnumerator3"))
  (Variables|Default|SetCenterArtIndex 1)
  (CallFunction|CenterArtUpdate _output_get))

(fn SearchArtSetIndex
  (params (Direction :type Integer) (StartIndex :type Integer))
  (bind _output_get (LocalVariables|SetDir Direction))
  (LocalVariables|SetNextIndex (+ _output_get StartIndex))
  (bind _result (Class|BPIControlCharacter|IsinAvailableArtRange(Message) (Variables|Default|GetMainCharacter) (LocalVariables|GetNextIndex)))
  (if _result
    (bind _result_2 (Class|BPIControlCharacter|IsAvailableArtPos(Message) (Variables|Default|GetMainCharacter) (LocalVariables|GetNextIndex)))
    (if _result_2
      (return (LocalVariables|GetNextIndex))
      (else
        (bind _artsetindex (CallFunction|SearchArtSetIndex (LocalVariables|GetDir) (LocalVariables|GetNextIndex)))
        (return _artsetindex)))
    (else
      (return -1))))

(fn UseSelectingArt
  (return 0))