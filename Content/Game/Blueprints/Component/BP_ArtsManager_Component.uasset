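; BP_ArtsManager_Component holds a character's set of available arts and resolves each to its ability.
; Initialize unpacks the supplied data into normal arts, talent art, escape, chain attack and draw weapon slots.
; One Use function per slot, indexed for normal arts, passes the stored art to UseArt.
; UseArt returns the ArtAbility from that art's data, leaving activation to the caller.
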(event EventTick
  (params (DeltaSeconds :type Float%20%28single-precision%29)))

(event EventInitialize
  (params (Data :type Available%20Arts%20Structure))
  (bind _output_get (Variables|Default|SetAvailables Data))
  (Variables|Default|SetNormalArts (.NormalArts (Utilities|Struct|BreakAvailableArts _output_get)))
  (Variables|Default|SetTalentArt (.TalentArt (Utilities|Struct|BreakAvailableArts _output_get)))
  (Variables|Default|SetEscape (.Escape (Utilities|Struct|BreakAvailableArts _output_get)))
  (Variables|Default|SetChainAttack (.ChainAttack (Utilities|Struct|BreakAvailableArts _output_get)))
  (Variables|Default|SetDraw%20Weapon (.DrawWeapon (Utilities|Struct|BreakAvailableArts _output_get))))

(fn UseArt
  (params (Art :type Object%20Object%20Reference))
  (bind _artdata (Class|BPIEquipedArt|GetData(Message) Art))
  (return (Variables|/Script/XenoLikeProject.ArtDataAsset|GetArtAbility _artdata)))

(fn UseChainAttack
  (bind _ability (CallFunction|UseArt (Variables|Default|GetChainAttack)))
  (return _ability))

(fn UseDrawWeapon
  (bind _ability (CallFunction|UseArt (Variables|Default|GetDraw%20Weapon)))
  (return _ability))

(fn UseEscape
  (bind _ability (CallFunction|UseArt (Variables|Default|GetEscape)))
  (return _ability))

(fn UseNormalArt
  (params (Idx :type Integer))
  (bind _ability (CallFunction|UseArt (Utilities|Array|Get(acopy) (Variables|Default|GetNormalArts) Idx)))
  (return _ability))

(fn UseTalentArt
  (bind _ability (CallFunction|UseArt (Variables|Default|GetTalentArt)))
  (return _ability))