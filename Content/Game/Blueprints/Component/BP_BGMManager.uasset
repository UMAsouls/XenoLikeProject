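; BP_BGMManager is a component that switches the game's background music between a calm normal track and a battle track.
; It drives an externally supplied audio component, applying a stored volume when that component is assigned.
; Battle start fades out, waits, then plays the battle track from an offset, with a BGMBattle flag checked to skip repeat triggers.
; Battle end fades out, clears the flag and fades the normal track back in.
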(event Custom|PlayNormalBGM
  (Variables|Default|SetBGMBattle false)
  (Audio|Components|Audio|SetSound (Variables|Default|GetAudio%20Comp) "/Game/Assets/Music/BGM/ファンタジー3-やすらぎ-.ファンタジー3-やすらぎ-")
  (Audio|Components|Audio|Play (Variables|Default|GetAudio%20Comp) 0.0))

(event Custom|SetAudioComponent
  (params (AudioComp :type Audio%20Component%20Object%20Reference))
  (Variables|Default|SetAudio%20Comp AudioComp)
  (Audio|Components|Audio|SetVolumeMultiplier (Variables|Default|GetAudio%20Comp) (Variables|Default|Getvolume) :!class /Script/Engine.AudioComponent))

(event Custom|OnBattleStart
  (if (not (Variables|Default|GetBGMBattle))
    (Audio|Components|Audio|FadeOut (Variables|Default|GetAudio%20Comp) 0.2 0.0 "Linear" :!class /Script/Engine.AudioComponent)
    (Utilities|FlowControl|Delay 0.8)
    (Audio|Components|Audio|SetSound (Variables|Default|GetAudio%20Comp) "/Game/Assets/Music/BGM/RPG_Battle_04.RPG_Battle_04")
    (Audio|Components|Audio|Play (Variables|Default|GetAudio%20Comp) 38.0)
    (Variables|Default|SetBGMBattle true)))

(event Custom|OnBattleEnd
  (Variables|Default|SetBGMBattle false)
  (Audio|Components|Audio|FadeOut (Variables|Default|GetAudio%20Comp) 0.8 0.0 "Linear" :!class /Script/Engine.AudioComponent)
  (Utilities|FlowControl|Delay 0.8)
  (Audio|Components|Audio|SetSound (Variables|Default|GetAudio%20Comp) "/Game/Assets/Music/BGM/ファンタジー3-やすらぎ-.ファンタジー3-やすらぎ-")
  (Audio|Components|Audio|FadeIn (Variables|Default|GetAudio%20Comp) 0.3 1.0 0.0 "Linear" :!class /Script/Engine.AudioComponent))

(event EventBeginPlay)

(event EventTick
  (params (DeltaSeconds :type Float%20%28single-precision%29)))