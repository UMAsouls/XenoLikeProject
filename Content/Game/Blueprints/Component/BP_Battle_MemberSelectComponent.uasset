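; Battle component that runs party member selection, moving a wrapping cursor across the members in the party subsystem.
; StartSelect stores the requesting getter and resets the index, and each move updates the highlight in the member status bar widget.
; Confirm passes the chosen member back to the getter and clears the highlight, while cancel clears it, resets the index and notifies the getter.
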(event Custom|UpdateSelect
  ;[0.15 0.15 0.15 0.5] 選択場所更新
  (Class|BPIMemberStatusBarUI|SetSelect(Message) (Class|WidgetRegisterSubsystem|GetWidget (Subsystems|GetWidgetRegisterSubsystem) "/Game/Game/Blueprints/WBP_MemberStatusBarUI.WBP_MemberStatusBarUI_C") (Variables|Default|GetSelectIdx)))

(event Custom|MemberSelectorMove
  (params (Dir :type Integer))
  ;[0.15 0.15 0.15 0.5] セレクターを動かす
  (bind _returnvalue (Class|PartySubsystem|GetPartyMemberCount (Subsystems|GetPartySubsystem)))
  (Variables|Default|SetSelectIdx (Class|KismetMathLibrary|Wrap (+ (Variables|Default|GetSelectIdx) (Class|KismetMathLibrary|SignOfInteger Dir)) -1 (- _returnvalue 1)))
  (CallFunction|UpdateSelect))

(event Custom|SelectCancel
  ;[0.15 0.15 0.15 0.5] セレクターを消す
  (Class|BPIMemberStatusBarUI|ClearSelect(Message) (Class|WidgetRegisterSubsystem|GetWidget (Subsystems|GetWidgetRegisterSubsystem) "/Game/Game/Blueprints/WBP_MemberStatusBarUI.WBP_MemberStatusBarUI_C"))
  (Variables|Default|SetSelectIdx 0)
  (Class|BPISelectMemberGetter|CancelSelect(Message) (Variables|Default|GetSelect%20Member%20Getter)))

(event Custom|StartSelect
  (params (SelectMemberGetter :type Object%20Object%20Reference))
  (Variables|Default|SetSelect%20Member%20Getter SelectMemberGetter)
  (Variables|Default|SetSelectIdx 0)
  (CallFunction|UpdateSelect))

(event Custom|ConfirmMember
  (bind _returnvalue (Class|PartySubsystem|GetPartyMember (Subsystems|GetPartySubsystem) (Variables|Default|GetSelectIdx)))
  (Class|BPISelectMemberGetter|Choose(Message) (Variables|Default|GetSelect%20Member%20Getter) _returnvalue)
  (Class|BPIMemberStatusBarUI|ClearSelect(Message) (Class|WidgetRegisterSubsystem|GetWidget (Subsystems|GetWidgetRegisterSubsystem) "/Game/Game/Blueprints/WBP_MemberStatusBarUI.WBP_MemberStatusBarUI_C")))

(event EventBeginPlay)

(event EventTick
  (params (DeltaSeconds :type Float%20%28single-precision%29)))