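; Manager that runs the party's chain attack, a turn-based sequence where living members act in rotation up to a maximum attack count.
; On start it switches party, player controller and enemies into chain attack mode via messages, then waits on gameplay tags until every member and the locked-on enemy are ready.
; It hands each turn to the player controller, skipping dead members, and reverts the mode at the end.
; GetChainAttackBonus scales linearly with attack count up to a cap.
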(event Custom|ChainAttackStart
  (bind _returnvalue (Class|PartySubsystem|GetPartyMembers (Subsystems|GetPartySubsystem)))
  (Utilities|FlowControl|Sequence
    (:then_0
      ;[0.15 0.15 0.15 0.5] 初期化
      (Variables|Default|SetAttackCount 0)
      (Variables|Default|SetMemberIdx 0)
      (Variables|Default|SetMemberChainAttackReady 0)
      (Variables|Default|SetEnemyChainAttackReady false)
      (Variables|Default|SetIsInChainAttack true))
    (:then_1
      ;[0.15 0.15 0.15 0.5] チェインアタック開始伝播
      (for _array_element _returnvalue
        (bind _result (Class|BPICharacter|GetIsDeath(Message) _array_element))
        (if (not _result)
          (Class|BPICharacter|ChangeChainAttackMode(Message) _array_element true)))
      (Class|BPICharacterController|OnChainAttackStart(Message) (Game|GetPlayerController 0))
      (for _array_element_2 (Variables|/Script/XenoLikeProject.EnemiesSubsystem|GetEnemies (Subsystems|GetEnemiesSubsystem))
        (Class|BPICharacter|ChangeChainAttackMode(Message) _array_element_2 true)))
    (:then_2
      ;[0.15 0.15 0.15 0.5] チェインアタックフェイズになるまで待つ
      (for _array_element_3 _returnvalue
        (bind _result_2 (Class|BPICharacter|GetIsDeath(Message) _array_element_3))
        (if _result_2
          (Math|Integer|IncrementInt (Variables|Default|GetMemberChainAttackReady) :!label _label)
          (elif (GameplayTags|HasMatchingGameplayTag _array_element_3 "(TagName=\"Chara.Phase.ChainAttack\")")
            (goto _label)
            (else
              (Ability|Tasks|WaitGameplayTagAddToActor _array_element_3 "(TagName=\"Chara.Phase.ChainAttack\")"
                (:Added
                  (Math|Integer|IncrementInt (Variables|Default|GetMemberChainAttackReady)
                    (:%20%20
                      (CallFunction|ChainAttackReady)))))))))
      (bind _target (Class|BPICharacter|GetCurrentLockonTarget(Message) (Game|Player|GetPlayerPawn 0)))
      (bind _returnvalue_2 (GameplayTags|HasMatchingGameplayTag(Message) _target "(TagName=\"Chara.Phase.ChainAttack\")"))
      (if _returnvalue_2
        (Variables|Default|SetEnemyChainAttackReady true)
        (CallFunction|ChainAttackReady)
        (else
          (Ability|Tasks|WaitGameplayTagAddToActor _target "(TagName=\"Chara.Phase.ChainAttack\")"
            (:Added
              (Variables|Default|SetEnemyChainAttackReady true)
              (CallFunction|ChainAttackReady))))))))

(event Custom|ChainAttackEnd
  (bind _returnvalue (Class|PartySubsystem|GetPartyMembers (Subsystems|GetPartySubsystem)))
  (for _array_element _returnvalue
    (bind _result (Class|BPICharacter|GetIsDeath(Message) _array_element))
    (if (not _result)
      (Class|BPICharacter|ChangeChainAttackMode(Message) _array_element false)))
  (Class|BPICharacterController|OnChainAttackEnd(Message) (Game|GetPlayerController 0))
  (for _array_element_2 (Variables|/Script/XenoLikeProject.EnemiesSubsystem|GetEnemies (Subsystems|GetEnemiesSubsystem))
    (Class|BPICharacter|ChangeChainAttackMode(Message) _array_element_2 false))
  (Variables|Default|SetIsInChainAttack false)
  (Variables|Default|SetAttackCount 0))

(event Custom|SelectNextMember
  (if (< (Variables|Default|GetAttackCount) (Variables|Default|GetMaxAttackCount))
    (bind _returnvalue (Class|PartySubsystem|GetPartyMemberCount (Subsystems|GetPartySubsystem)))
    (Variables|Default|SetMemberIdx (Class|KismetMathLibrary|Wrap (+ (Variables|Default|GetMemberIdx) 1) -1 (- _returnvalue 1)))
    (CallFunction|IndexMemberSet)
    (else
      (CallFunction|ChainAttackEnd))))

(event Custom|IndexMemberSet
  (bind _returnvalue (Class|PartySubsystem|GetPartyMember (Subsystems|GetPartySubsystem) (Variables|Default|GetMemberIdx)))
  (bind _result (Class|BPICharacter|GetIsDeath(Message) _returnvalue))
  (if _result
    (CallFunction|SelectNextMember)
    (else
      (Math|Integer|IncrementInt (Variables|Default|GetAttackCount)
        (:%20%20
          (Class|BPICharacterController|SetChainAttackMember(Message) (Game|GetPlayerController 0) _returnvalue))))))

(event Custom|ChainAttackReady
  (bind _returnvalue (Class|PartySubsystem|GetPartyMemberCount (Subsystems|GetPartySubsystem)))
  (if (and (Variables|Default|GetEnemyChainAttackReady) (== _returnvalue (Variables|Default|GetMemberChainAttackReady)))
    (CallFunction|IndexMemberSet)))

(event EventBeginPlay)

(event EventTick
  (params (DeltaSeconds :type Float%20%28single-precision%29)))

(fn GetChainAttackBonus
  (return (+ (LocalVariables|GetFirstBonus) (* (LocalVariables|GetBonusBase) (- (Math|Integer|Min(Integer) (LocalVariables|GetMaxBonusCount) (Variables|Default|GetAttackCount)) 1)))))