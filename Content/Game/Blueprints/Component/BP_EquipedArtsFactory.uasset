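; Factory that builds a character's set of equipped arts from art data, covering normal, talent, escape, chain attack and draw weapon slots.
; MakeAvailableArts spawns an actor per art, using BP_EquipedArt for normal, BP_EquipedTalentArt for talent and chain attack, and BP_EquipedNonRecastArt for escape and draw weapon.
; Each actor receives its data through InitializeMessage.
; The normal arts array is filled by a recursive function rather than a loop.
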(event EventBeginPlay)

(event EventTick
  (params (DeltaSeconds :type Float%20%28single-precision%29)))

(fn MakeAvailableArts
  (params (NormalArtDatas :type Array%20of%20Art%20Data%20Asset%20Object%20References) (TalentArtData :type Art%20Data%20Asset%20Object%20Reference) (EscapeData :type Art%20Data%20Asset%20Object%20Reference) (ChainAttackData :type Art%20Data%20Asset%20Object%20Reference) (DrawWeaponData :type Art%20Data%20Asset%20Object%20Reference))
  (return (Utilities|Struct|MakeAvailableArts (CallFunction|MakeNormalEquipedArts NormalArtDatas) (CallFunction|MakeEquipedArt "/Game/Game/Blueprints/BP_EquipedTalentArt.BP_EquipedTalentArt_C" TalentArtData) (CallFunction|MakeEquipedArt "/Game/Game/Blueprints/BP_EquipedNonRecastArt.BP_EquipedNonRecastArt_C" EscapeData) (CallFunction|MakeEquipedArt "/Game/Game/Blueprints/BP_EquipedTalentArt.BP_EquipedTalentArt_C" ChainAttackData) (CallFunction|MakeEquipedArt "/Game/Game/Blueprints/BP_EquipedNonRecastArt.BP_EquipedNonRecastArt_C" DrawWeaponData))))

(fn MakeEquipedArt
  (params (Type :type Actor%20Class%20Reference) (ArtData :type Art%20Data%20Asset%20Object%20Reference))
  (bind _returnvalue (Game|SpawnActorfromClass Type (Math|Transform|MakeTransform "0, 0, 0") "Undefined" "MultiplyWithRoot" 0 0))
  (Class|BPIEquipedArt|Initialize(Message) _returnvalue ArtData)
  (return _returnvalue))

(fn MakeNormalEquipedArtsRecrusion
  (params (Arts :type Array%20of%20Art%20Data%20Asset%20Object%20References) (Index :type Integer) (SettingArray :type Array%20of%20Object%20Object%20References))
  (LocalVariables|SetLocalArts Arts)
  (LocalVariables|SetLocalIndex Index)
  (LocalVariables|SetLocalSettingArray SettingArray)
  (if (Utilities|Array|IsValidIndex (LocalVariables|GetLocalArts) (LocalVariables|GetLocalIndex))
    (Utilities|Array|SetArrayElem (LocalVariables|GetLocalSettingArray) (LocalVariables|GetLocalIndex) (CallFunction|MakeEquipedArt "/Game/Game/Blueprints/BP_EquipedArt.BP_EquipedArt_C" (Utilities|Array|Get(acopy) (LocalVariables|GetLocalArts) (LocalVariables|GetLocalIndex))) true)
    (bind _normalequipedarts (CallFunction|MakeNormalEquipedArtsRecrusion (LocalVariables|GetLocalArts) (+ (LocalVariables|GetLocalIndex) 1) (LocalVariables|GetLocalSettingArray)))
    (return _normalequipedarts)
    (else
      (return (LocalVariables|GetLocalSettingArray)))))

(fn MakeNormalEquipedArts
  (params (Arts :type Array%20of%20Art%20Data%20Asset%20Object%20References))
  (bind _normalequipedarts (CallFunction|MakeNormalEquipedArtsRecrusion Arts))
  (return _normalequipedarts))