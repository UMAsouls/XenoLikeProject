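; Hate (threat) component that tracks how much hate its owner holds toward each party member and reports the highest-hate member.
; It binds to party death and rebirth events and the owner's attribute-set damage delegate.
; MemberUpdate rebuilds the map with living members at zero hate, also running when damage finds it empty.
; Damage times a multiplier adds clamped hate to mapped attackers only; battle end clears the map.
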(event Custom|OnBattleBegin)

(event Custom|OnDamaged
  (params (Damage :type Float%20%28double-precision%29) (SourceActor :type Actor%20Object%20Reference))
  (if (Utilities|Map|IsEmpty (Variables|Default|GetHateMap))
    (CallFunction|MemberUpdate))
  (CallFunction|AddHate SourceActor (* Damage (Variables|Default|Get%20DamageHateParam))))

(event Custom|AddHate
  (params (Member :type Actor%20Object%20Reference) (Hate :type Float%20%28double-precision%29))
  (bind _hatemap (Variables|Default|GetHateMap))
  (bind (_value _returnvalue) (Utilities|Map|Find _hatemap Member))
  (if _returnvalue
    (Utilities|Map|Add (Variables|Default|GetHateMap) Member (Math|Float|Clamp(Float) (+ _value Hate) 0.0 9999.0))))

(event Custom|MemberUpdate
  (Utilities|Map|Clear (Variables|Default|GetHateMap))
  (bind _returnvalue (Class|PartySubsystem|GetPartyMembers (Subsystems|GetPartySubsystem)))
  (for _array_element _returnvalue
    (bind _result (Class|BPICharacter|GetIsDeath(Message) _array_element))
    (if (not _result)
      (Utilities|Map|Add (Variables|Default|GetHateMap) _array_element 0.0))))

(event Custom|OnBattleEnd
  (Utilities|Map|Clear (Variables|Default|GetHateMap)))

(event EventBeginPlay
  (EventDispatchers|BindEventtoMemberDeathDelegate (Subsystems|GetPartySubsystem) (EventDispatchers|CreateEvent :!event Custom|MemberUpdate))
  (EventDispatchers|BindEventtoMemberRebirthDelegate (Subsystems|GetPartySubsystem) (EventDispatchers|CreateEvent :!event Custom|MemberUpdate))
  (bind _returnvalue (GameplayAttributes|GetAttributeSet (Ability|GetAbilitySystemComponent (Components|GetOwner)) "/Script/XenoLikeProject.XenoCharacterAttributeSet"))
  (EventDispatchers|BindEventtoOnDamage _returnvalue (EventDispatchers|CreateEvent :!event Custom|OnDamaged)))

(event EventTick
  (params (DeltaSeconds :type Float%20%28single-precision%29)))

(fn GetBestHateMember
  (bind _values (Utilities|Map|Values (Variables|Default|GetHateMap)))
  (return (.Key (Utilities|Map|GetKeyValueByIndex (Variables|Default|GetHateMap) (.IndexOfMaxValue (Math|Float|MaxOfFloatArray _values))))))