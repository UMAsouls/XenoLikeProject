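; Component that shows and hides the party leader's lock-on HUD: member status bars, enemy status bar, arts palette and party gauge.
; SetLeader binds to the leader's lock-on and unlock events, which create or remove these widgets.
; Status bars are assigned to PartySubsystem members, and the palette is filled from the leader's normal and center arts.
; All widgets except the palette are registered with WidgetRegisterSubsystem.
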(event Custom|OnUnLockOn
  (Utilities|IsValid (Variables|Default|GetMemberStatusBarUI)
    (:Is%20Valid
      (Class|BPIWidgetRemoveAnimation|RemoveAnimation(Message) (Variables|Default|GetMemberStatusBarUI))
      (Class|WidgetRegisterSubsystem|RemoveWidget (Subsystems|GetWidgetRegisterSubsystem) "/Game/Game/Blueprints/WBP_EnemyStatusBar.WBP_EnemyStatusBar_C")
      (CallFunction|RemoveArtsPalette)
      (CallFunction|RemovePartyGage))))

(event Custom|SetLeader
  (params (%20Leader :type BP%20Main%20Character%20Object%20Reference))
  (Variables|Default|SetLeader %20Leader)
  (Utilities|FlowControl|Sequence
    (:then_0
      (EventDispatchers|BindEventtoOnUnLockonTarget (Variables|Default|GetLeader) (delegate Custom|OnUnLockOn)))
    (:then_1
      (EventDispatchers|BindEventtoOnNewTargetLockon (Variables|Default|GetLeader) (delegate Custom|OnLockOn)))))

(event Custom|ShowEnemyStatusBar
  ;[0.15 0.15 0.15 0.5] 敵のStatusBar表示
  (Utilities|IsValid (Variables|Default|GetEnemyStatusBar)
    (:Is%20Valid
      _)
    (:Is%20Not%20Valid
      (bind _returnvalue (UserInterface|CreateWidget "/Game/Game/Blueprints/WBP_EnemyStatusBar.WBP_EnemyStatusBar_C" 0 (Variables|Default|GetLeader)))
      (Variables|Default|SetEnemyStatusBar _returnvalue)))
  (if (not (UserInterface|Viewport|IsinViewport (Variables|Default|GetEnemyStatusBar)))
    (UserInterface|Viewport|AddtoViewport (Variables|Default|GetEnemyStatusBar) 0)
    (Class|WidgetRegisterSubsystem|RegisterWidget (Subsystems|GetWidgetRegisterSubsystem) "/Game/Game/Blueprints/WBP_EnemyStatusBar.WBP_EnemyStatusBar_C" (Variables|Default|GetEnemyStatusBar))))

(event Custom|RemoveArtsPalette
  ;[0.15 0.15 0.15 0.5] アーツパレット関連(Unbind処理も作らなきゃ)
  (Utilities|IsValid (Variables|Default|GetArtsPalette)
    (:Is%20Valid
      (Widget|RemovefromParent (Variables|Default|GetArtsPalette)))))

(event Custom|OnLockOn
  (CallFunction|ShowMemberStatusBar)
  (CallFunction|ShowEnemyStatusBar)
  (CallFunction|ShowArtsPalette)
  (CallFunction|ShowPartyGage))

(event Custom|ShowMemberStatusBar
  ;[0.15 0.15 0.15 0.5] 味方のstatusBar表示
  (bind _returnvalue (UserInterface|CreateWidget "/Game/Game/Blueprints/WBP_MemberStatusBarUI.WBP_MemberStatusBarUI_C"))
  (Variables|Default|SetMemberStatusBarUI _returnvalue)
  (bind _returnvalue_2 (Class|PartySubsystem|GetPartyMembers (Subsystems|GetPartySubsystem)))
  (for (_array_element _array_index) _returnvalue_2
    (Utilities|IsValid _array_element
      (:Is%20Valid
        (Class|BPIPlayer|SetStatusBar(Message) _array_element (Default|GetStatusBar _returnvalue _array_index)))))
  (if (not (UserInterface|Viewport|IsinViewport (Variables|Default|GetMemberStatusBarUI)))
    (UserInterface|Viewport|AddtoViewport (Variables|Default|GetMemberStatusBarUI) 0)
    (Class|WidgetRegisterSubsystem|RegisterWidget (Subsystems|GetWidgetRegisterSubsystem) "/Game/Game/Blueprints/WBP_MemberStatusBarUI.WBP_MemberStatusBarUI_C" (Variables|Default|GetMemberStatusBarUI))))

(event Custom|SetArtsToUI
  (params (Member :type Actor%20Object%20Reference))
  ;[0.15 0.15 0.15 0.5] アーツパレット関連(Unbind処理も作らなきゃ)
  (bind _normalarts (Class|BPIControlCharacter|GetNormalArts(Message) Member))
  (Default|SetNormalArts (Variables|Default|GetArtsPalette) _normalarts 0 Member)
  (bind _centerart (Class|BPIControlCharacter|GetCenter(Message) Member))
  (Default|SetCenterArt (Variables|Default|GetArtsPalette) _centerart Member))

(event Custom|ShowArtsPalette
  ;[0.15 0.15 0.15 0.5] アーツパレット関連(Unbind処理も作らなきゃ)
  ;;[0.15 0.15 0.15 0.5] アーツパレット作成
  (Utilities|FlowControl|Sequence
    (:then_0
      (Utilities|IsValid (Variables|Default|GetArtsPalette)
        (:Is%20Valid
          _)
        (:Is%20Not%20Valid
          (bind _returnvalue (UserInterface|CreateWidget "/Game/Game/Blueprints/WBP_ArtsPalette.WBP_ArtsPalette_C"))
          (Variables|Default|SetArtsPalette _returnvalue)))
      (if (not (UserInterface|Viewport|IsinViewport (Variables|Default|GetArtsPalette)))
        (UserInterface|Viewport|AddtoViewport (Variables|Default|GetArtsPalette) 0)))
    (:then_1
      ;;;[0.15 0.15 0.15 0.5] アーツパレットの設定
      (EventDispatchers|BindEventtoOnCenterArtUpdate (Variables|Default|GetLeader) (EventDispatchers|CreateEvent (Variables|Default|GetArtsPalette) :!event SetCenterArt))
      (CallFunction|SetArtstoUI (Variables|Default|GetLeader))
      (Default|CallEDonArtPaletteShow (Variables|Default|GetArtsPalette)))))

(event Custom|ShowPartyGage
  (bind _returnvalue (UserInterface|CreateWidget "/Game/Game/Blueprints/Widget/WBP_PartyGage.WBP_PartyGage_C"))
  (bind _output_get (Variables|Default|SetPartyGageWidget _returnvalue))
  (if (not (UserInterface|Viewport|IsinViewport _output_get))
    (UserInterface|Viewport|AddtoViewport (Variables|Default|GetPartyGageWidget) 1)
    (Class|WidgetRegisterSubsystem|RegisterWidget (Subsystems|GetWidgetRegisterSubsystem) "/Game/Game/Blueprints/Widget/WBP_PartyGage.WBP_PartyGage_C" (Variables|Default|GetPartyGageWidget))
    (Widget|SetVisibility (Variables|Default|GetPartyGageWidget) "Visible")))

(event Custom|RemovePartyGage
  (Widget|RemovefromParent (Variables|Default|GetPartyGageWidget)))

(event EventBeginPlay)

(event EventTick
  (params (DeltaSeconds :type Float%20%28single-precision%29)))