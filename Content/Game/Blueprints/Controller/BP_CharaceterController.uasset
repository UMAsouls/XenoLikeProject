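; AI controller for characters that drives their behavior through a Blackboard and Behavior Tree.
; On BeginPlay it sets up the Blackboard, starts the tree logic, then injects Fight and Normal behavior assets as dynamic subtrees by gameplay tag.
; A Damaged event raises a Blackboard flag so the tree can react to hits.
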(event EventBeginPlay
  ;[0.15 0.15 0.15 0.5] Normal・Fight状態のツリーをセット
  (Class|AIController|UseBlackboard (Variables|Default|GetBlackBoardAsset))
  (AI|Logic|StartLogic (Variables|Default|GetBehaviorTree))
  (Class|BehaviorTreeComponent|SetDynamicSubtree (Variables|Default|GetBehaviorTree) "(TagName=\"BehaviorTree.Character.Fight\")" (Variables|Default|GetFightBehavior))
  (Class|BehaviorTreeComponent|SetDynamicSubtree (Variables|Default|GetBehaviorTree) "(TagName=\"BehaviorTree.Character.Normal\")" (Variables|Default|GetNormalBehavior)))

(event EventTick
  (params (DeltaSeconds :type Float%20%28single-precision%29)))

(event EventDamaged
  (params (Damage :type Float%20%28double-precision%29))
  (AI|Components|Blackboard|SetValueasBool (Variables|Default|GetBlackboard) (Utilities|Name|MakeLiteralName "Damaged") true))

(fn ConstructionScript)