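; BP_MemberController is a controller for a party member that feeds player and combat state into its Blackboard.
; On BeginPlay it stores the player pawn as PlayerActor and registers two callbacks with the party subsystem.
; The draw-weapon and unequip callbacks set the Fight key true and false, so combat state follows those events without polling on Tick.
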(event Custom|DrawWeaponDelegate_Event
  (AI|Components|Blackboard|SetValueasBool (Variables|Default|GetBlackboard) (Utilities|Name|MakeLiteralName "Fight") true))

(event Custom|UnEquipDelegate_Event
  (AI|Components|Blackboard|SetValueasBool (Variables|Default|GetBlackboard) (Utilities|Name|MakeLiteralName "Fight") false))

(event EventBeginPlay
  (|CallParentFunction)
  (AI|Components|Blackboard|SetValueasObject (Variables|Default|GetBlackboard) (Utilities|Name|MakeLiteralName "PlayerActor") (Game|Player|GetPlayerPawn 0))
  (EventDispatchers|AssignDrawWeaponDelegate (Subsystems|GetPartySubsystem) (delegate Custom|DrawWeaponDelegate_Event))
  (EventDispatchers|AssignUnEquipDelegate (Subsystems|GetPartySubsystem) (delegate Custom|UnEquipDelegate_Event)))

(event EventTick
  (params (DeltaSeconds :type Float%20%28single-precision%29))
  (|CallParentFunction DeltaSeconds) ; This node is disabled and will not be called.\nDrag off pins to build functionality.
)

(fn ConstructionScript
  (|CallParentFunction))