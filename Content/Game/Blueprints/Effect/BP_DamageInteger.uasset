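; BP_DamageInteger is a floating damage number actor that shows a value in its Num widget component.
; External callers set the widget class through SetWidget and pass the amount through SetDamage, which forwards it to the widget's SetDamageMessage.
; Tick moves the widget upward by UpSpeed each frame without delta-time scaling.
; After DisplayTime, the DestroyTimer timeline drives the widget's opacity, then the actor destroys itself.
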(event EventBeginPlay
  (Utilities|FlowControl|Delay (Variables|Default|GetDisplayTime))
  (bind _alpha (Timeline|DestroyTimer Play)
    (:Update
      (Widget|SetRenderOpacity (UserInterface|GetWidget (Variables|Default|GetNum)) _alpha))
    (:Finished
      (Actor|DestroyActor))))

(event Collision|EventActorBeginOverlap
  (params (OtherActor :type Actor%20Object%20Reference)))

(event EventTick
  (params (DeltaSeconds :type Float%20%28single-precision%29))
  (Transformation|AddRelativeLocation (Variables|Default|GetNum) (Math|Vector|MakeVector 0.0 0.0 (Variables|Default|Get%20UpSpeed)) false false))

(event EventSetDamage
  (params (damage :type Float%20%28double-precision%29))
  (Class|BPIDamageInteger|SetDamage(Message) (UserInterface|GetWidget (Variables|Default|GetNum)) damage))

(event EventSetWidget
  (params (wid :type User%20Widget%20Class%20Reference))
  (bind _returnvalue (UserInterface|CreateWidget wid))
  (UserInterface|SetWidget (Variables|Default|GetNum) _returnvalue))

(fn ConstructionScript)