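; BP_AttackHitStrategy decides whether an ability attack from a Source lands on a Target.
; JudgeHit checks the target's ability system component against the InvalidAttackTag list and, on the first match, reports the miss with that tag through the source's XenoCharacterAttributeSet.
; It returns false for a miss and true otherwise, leaving propagation of the hit result to Gameplay Effects.
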(fn JudgeHit
  (params (Source :type Actor%20Object%20Reference) (Target :type Actor%20Object%20Reference))
  (for _array_element (LocalVariables|GetInvalidAttackTag)
    (if (GameplayTags|HasMatchingGameplayTag (Ability|GetAbilitySystemComponent Target) _array_element)
      (LocalVariables|SetMissResultTag _array_element)
      (bind _returnvalue (GameplayAttributes|GetAttributeSet (Ability|GetAbilitySystemComponent Source) "/Script/XenoLikeProject.XenoCharacterAttributeSet"))
      (Default|CallOnAttackMissed _returnvalue (GameplayTags|MakeGameplayTagContainerfromTag (LocalVariables|GetMissResultTag)))
      (return false)))
  (return true) ; 攻撃の結果を伝播するのはGEに任せる
)