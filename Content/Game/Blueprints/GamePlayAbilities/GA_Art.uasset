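; Gameplay ability for character Arts: commits cost, picks targets by selection type (lock-on, self, area, forward cone, party member), then plays a montage.
; Montage hit events spawn strategy-placed VFX and apply tag-gated effects through optional hit strategies, with chain-attack-scaled magnitudes.
; Recast uses either talent-gauge activation or a standby effect removed at ability end, deferred during chain attacks.
; End-of-art effects apply to the caster.
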(event Custom|AnimationStart
  ;[0.15 0.15 0.15 0.5] アニメーション処理
  (Ability|ApplyGameplayEffectToOwner "/Game/Game/Blueprints/GamePlayEffects/Battle/GE_MoveStop.GE_MoveStop_C")
  (|PlayMontageandWaitProxy "None" (Variables|Default|GetMontage%20to%20Play) 1.0 "None" true 1.0 0.0 true
    (:then
      (bind _asynctaskproxy (Ability|Tasks|WaitGameplayEvent "(TagName=\"Event.Montage.Attack.Hit\")" 0)
        (:then
          (Variables|Default|SetAsync%20Task _asynctaskproxy))
        (:EventReceived
          (CallFunction|OnHit))))
    (:OnCompleted
      (Ability|EndAbility))
    (:OnInterrupted
      (Ability|CancelAbility))))

(event Custom|OnHit
  ;[0.15 0.15 0.15 0.5] アーツ発動タイミングになったときのエフェクト発動処理
  (CallFunction|SpawnVFX (Utilities|Array|Get(acopy) (Variables|Default|GetAtrVFXs) (Variables|Default|GetVFXIdx)) (Variables|Default|GetTargetList))
  (for _array_element (Variables|Default|GetTargetList)
    (Variables|Default|SetTarget _array_element)
    (for _array_element_2 (Variables|Default|GetArtEffects)
      (if (Utilities|IsEffectApplyable (.TargetRequiredTag (Utilities|Struct|BreakST_ArtEffect _array_element_2)) (.SourceRequiredTag (Utilities|Struct|BreakST_ArtEffect _array_element_2)) (Variables|Default|GetTarget))
        (CallFunction|ApplyEffect (.ApplyEffect (Utilities|Struct|BreakST_ArtEffect _array_element_2)) (Variables|Default|GetTarget) (.SetByCallers (Utilities|Struct|BreakST_ArtEffect _array_element_2))))))
  (Variables|Default|SetVFXIdx (Class|KismetMathLibrary|Wrap (+ (Variables|Default|GetVFXIdx) 1) -1 (- (Utilities|Array|Length (Variables|Default|GetAtrVFXs)) 1))))

(event Custom|AroundSelect
  (params (Center :type Actor%20Object%20Reference) (EnemySelect :type Boolean) (Radius :type Float%20%28double-precision%29) (Angle :type Float%20%28double-precision%29))
  (bind _returnvalue (Transformation|GetActorLocation Center))
  ;[0.15 0.15 0.15 0.5] アーツ対象選択処理
  ;;[0.15 0.15 0.15 0.5] 範囲選択
  (bind _outhits (Collision|MultiSphereTraceForObjects _returnvalue _returnvalue Radius (Utilities|Array|MakeArray "ObjectTypeQuery3") false 0 "None" false))
  (for _array_element _outhits
    (if (Utilities|IsinAngle Center (.HitActor (Collision|BreakHitResult _array_element)) Angle)
      (bind _result (CallFunction|IsSameType (Ability|GetAvatarActorfromActorInfo) (.HitActor (Collision|BreakHitResult _array_element)) EnemySelect))
      (if _result
        (bind _result_2 (CallFunction|IsTargetHitable (.HitActor (Collision|BreakHitResult _array_element))))
        (if _result_2
          (Utilities|Array|Add (Variables|Default|GetTargetList) (.HitActor (Collision|BreakHitResult _array_element))))))))

(event Custom|SourceAroundMemberSelect
  ;[0.15 0.15 0.15 0.5] アーツ対象選択処理
  (CallFunction|AroundSelect (Ability|GetAvatarActorfromActorInfo) false (Variables|Default|GetArtRange) 3.6e+02)
  (CallFunction|AnimationStart))

(event Custom|SourceAroundEnemySelect
  ;[0.15 0.15 0.15 0.5] アーツ対象選択処理
  (CallFunction|AroundSelect (Ability|GetAvatarActorfromActorInfo) true (Variables|Default|GetArtRange) 3.6e+02)
  (CallFunction|SingleTargetSelect))

(event Custom|SourceForwardEnemySelect
  ;[0.15 0.15 0.15 0.5] アーツ対象選択処理
  (CallFunction|AroundSelect (Ability|GetAvatarActorfromActorInfo) true (Variables|Default|GetArtRange) 9e+01)
  (CallFunction|SingleTargetSelect))

(event Custom|RecastStart
  ;[0.15 0.15 0.15 0.5] リキャスト開始処理
  (if (not (Variables|Default|GetTalentArtFlag))
    (bind _returnvalue (GameplayTags|HasMatchingGameplayTag(Message) (Ability|GetAvatarActorfromActorInfo) "(TagName=\"Chara.Phase.ChainAttack\")"))
    (if _returnvalue
      (Ability|Tasks|WaitGameplayTagRemoveFromActor (Ability|GetAvatarActorfromActorInfo) "(TagName=\"Chara.Phase.ChainAttack\")" true
        (:Removed
          (Ability|RemoveGameplayEffectFromOwnerWithHandle (Variables|Default|GetActiveCooldownStandbyEffectSpec))))
      (else
        (bind _returnvalue_2 (Ability|GameplayEffect|GetActiveGameplayEffectStackCount (Variables|Default|GetActiveCooldownStandbyEffectSpec)))
        (if (> _returnvalue_2 0)
          (Ability|RemoveGameplayEffectFromOwnerWithHandle (Variables|Default|GetActiveCooldownStandbyEffectSpec))
          (Ability|CommitAbilityCooldown false))))))

(event Custom|MemberSelect
  ;[0.15 0.15 0.15 0.5] アーツ対象選択処理
  ;;[0.15 0.15 0.15 0.5] メンバー選択処理
  (Utilities|IsValid (AI|GetAIController (Ability|GetAvatarActorfromActorInfo))
    (:Is%20Not%20Valid
      (Class|BPICharacterController|BattleMemberSelectStart(Message) (Game|GetPlayerController 0) self))))

(event Custom|ApplyEffect
  (params (Effect :type Gameplay%20Effect%20Class%20Reference) (Target :type Actor%20Object%20Reference) (SetByCallers :type Array%20of%20ST%20Art%20Set%20by%20Caller%20Structures))
  (bind _hitstrategies (Variables|Default|GetHitStrategies))
  (bind (_value _returnvalue) (Utilities|Map|Find _hitstrategies Effect))
  ;[0.15 0.15 0.15 0.5] アーツ発動タイミングになったときのエフェクト発動処理
  (if _returnvalue
    (bind _returnvalue_2 (Game|ConstructObjectfromClass _value))
    (bind _result (Default|JudgeHit _returnvalue_2 (Ability|GetAvatarActorfromActorInfo) Target))
    (if _result
      ;;[0.15 0.15 0.15 0.5] setbycallerをするところ
      (Variables|Default|SetEffectSpec (GameplayEffects|MakeOutgoingSpec :self (Ability|GetAbilitySystemComponentfromActorInfo) :GameplayEffectClass Effect) :!label _label)
      (for _array_element SetByCallers
        (if (Utilities|IsEffectApplyable (.TargetRequiredTag (Utilities|Struct|BreakST_ArtSetByCaller _array_element)) (.SourceRequiredTag (Utilities|Struct|BreakST_ArtSetByCaller _array_element)) Target)
          (bind _returnvalue_3 (Ability|GameplayEffect|AssignTagSetbyCallerMagnitude (Variables|Default|GetEffectSpec) (.CallerTag (Utilities|Struct|BreakST_ArtSetByCaller _array_element)) (* (.CallerMagnitude (Utilities|Struct|BreakST_ArtSetByCaller _array_element)) (Math|Float|Max(Float) (* (.ChainAttackEffectable (Utilities|Struct|BreakST_ArtSetByCaller _array_element)) (Default|GetChainAttackBonus (Actor|GetComponentbyClass (Game|GetGameMode) "/Game/Game/Blueprints/Component/BP_ChainAttackManager.BP_ChainAttackManager_C"))) 1.0))))
          (Variables|Default|SetEffectSpec _returnvalue_3)))
      (GameplayEffects|ApplyGameplayEffectSpecToTarget (Variables|Default|GetEffectSpec) (Ability|TargetData|AbilityTargetDatafromActor Target)))
    (else
      (goto _label))))

(event Custom|SingleTargetSelect
  ;[0.15 0.15 0.15 0.5] アーツ対象選択処理
  ;;[0.15 0.15 0.15 0.5] LockOnTargetを選択する処理
  (bind _target (Class|BPICharacter|GetCurrentLockonTarget(Message) (Ability|GetAvatarActorfromActorInfo)))
  (Utilities|IsValid _target
    (:Is%20Valid
      (if (< (Utilities|Array|FindItem (Variables|Default|GetTargetList) _target) 0)
        (bind _result (CallFunction|IsTargetHitable _target))
        (if _result
          (Utilities|Array|Add (Variables|Default|GetTargetList) _target)
          (CallFunction|AnimationStart))
        (else
          (CallFunction|AnimationStart))))
    (:Is%20Not%20Valid
      (Ability|CancelAbility))))

(event Custom|SourceSelect
  ;[0.15 0.15 0.15 0.5] アーツ対象選択処理
  ;;[0.15 0.15 0.15 0.5] 自分自身を選択する処理
  (Utilities|Array|Add (Variables|Default|GetTargetList) (Ability|GetAvatarActorfromActorInfo))
  (CallFunction|AnimationStart))

(event Custom|ArtLastEffect
  (for _array_element (Variables|Default|GetArtLastEffects)
    (if (Utilities|IsEffectApplyable (.TargetRequiredTag (Utilities|Struct|BreakST_ArtEffect _array_element)) (.SourceRequiredTag (Utilities|Struct|BreakST_ArtEffect _array_element)) (Ability|GetAvatarActorfromActorInfo))
      (CallFunction|ApplyEffect (.ApplyEffect (Utilities|Struct|BreakST_ArtEffect _array_element)) (Ability|GetAvatarActorfromActorInfo) (.SetByCallers (Utilities|Struct|BreakST_ArtEffect _array_element))))))

(event Custom|TargetAroundEnemySelect
  ;[0.15 0.15 0.15 0.5] アーツ対象選択処理
  (bind _target (Class|BPICharacter|GetCurrentLockonTarget(Message) (Ability|GetAvatarActorfromActorInfo)))
  (CallFunction|AroundSelect _target true 5e+02 3.6e+02)
  (CallFunction|AnimationStart))

(event Custom|SpawnVFX
  (params (vfx :type ST%20Art%20VFX%20Structure) (Target :type Array%20of%20Actor%20Object%20References))
  (bind (_vfx _spawnstrategy _se _volume) (Utilities|Struct|BreakST_ArtVFX vfx))
  (bind _returnvalue (Game|ConstructObjectfromClass _spawnstrategy))
  (if (Utilities|Array|IsNotEmpty (Default|CalculateSpawnPlace _returnvalue 0 (Ability|GetAvatarActorfromActorInfo)))
    (for _array_element (Default|CalculateSpawnPlace _returnvalue 0 (Ability|GetAvatarActorfromActorInfo))
      (Game|SpawnActorfromClass _vfx _array_element "Undefined" "MultiplyWithRoot" 0 0)
      (Audio|PlaySoundatLocation _se (Math|Transform|TransformLocation _array_element "0, 0, 0") "0, 0, 0" _volume 1.0 0.0 0 0 0 0))))

(event Ability|EventActivateAbility
  (bind _returnvalue (Ability|CommitAbilityCost false))
  (if _returnvalue
    (bind _asbp_xeno_project_character (Utilities|Casting|CastToBP_XenoProjectCharacter (Ability|GetAvatarActorfromActorInfo))
      (:then
        (Default|LookatLockonTargetNow _asbp_xeno_project_character)
        (Default|CallEDonArtUse _asbp_xeno_project_character))
      (:CastFailed
        _))
    (if (Variables|Default|GetTalentArtFlag)
      (Abilities|TryActivateAbilitybyClass (Ability|GetAbilitySystemComponentfromActorInfo) "/Game/Game/Blueprints/GamePlayAbilities/GA_TalentArtRecast.GA_TalentArtRecast_C" true)
      (else
        (bind _returnvalue_2 (Ability|ApplyGameplayEffectSpecToOwner (Variables|Default|GetCooldownStandbyEffectSpec)))
        (Variables|Default|SetActiveCooldownStandbyEffectSpec _returnvalue_2)))
    (Utilities|Array|Clear (Variables|Default|GetTargetList))
    (switch Utilities|FlowControl|Switch|SwitchonEArtTargetSelectType (Variables|Default|GetArtTargetSelectType)
      (:NewEnumerator0
        (CallFunction|SingleTargetSelect))
      (:NewEnumerator1
        (CallFunction|TargetAroundEnemySelect))
      (:NewEnumerator2
        (CallFunction|SourceSelect))
      (:NewEnumerator3
        (CallFunction|SourceAroundEnemySelect))
      (:NewEnumerator4
        (CallFunction|MemberSelect))
      (:NewEnumerator5
        (CallFunction|SourceForwardEnemySelect))
      (:NewEnumerator6
        (CallFunction|SourceAroundMemberSelect)))
    (else
      (Ability|CancelAbility))))

(event Ability|EventOnEndAbility
  (params (bWasCancelled :type Boolean))
  (CallFunction|RecastStart)
  (Ability|RemoveGameplayEffectFromOwnerWithGrantedTags "(GameplayTags=((TagName=\"Chara.State.Movement.Stop\")))")
  (CallFunction|ArtLastEffect)
  (Utilities|IsValid (Variables|Default|GetAsync%20Task)
    (:Is%20Valid
      (GameplayTasks|EndTask (Variables|Default|GetAsync%20Task)))))

(event EventSetRecastTag
  (params (RecastTag :type Gameplay%20Tag%20Structure))
  ;[0.15 0.15 0.15 0.5] リキャスト設定処理
  (bind _output_get (Variables|Default|SetRecastTag RecastTag))
  (Variables|Default|SetCooldownTags (GameplayTags|MakeGameplayTagContainerfromTag _output_get))
  (if (GameplayTags|MatchesTag (Variables|Default|GetRecastTag) "(TagName=\"Art.Cooldown.Talent\")" true)
    (Variables|Default|SetTalentArtFlag true)
    (bind _returnvalue (Ability|GameplayEffect|AssignTagSetbyCallerMagnitude (GameplayEffects|MakeOutgoingSpec :self (Ability|GetAbilitySystemComponentfromActorInfo) :GameplayEffectClass "/Game/Game/Blueprints/GamePlayEffects/GE_SetTalentArtGage.GE_SetTalentArtGage_C") "(TagName=\"Data.Cooldown.Talent\")" (Variables|Default|Get%20TalentArtRecast)))
    (Ability|ApplyGameplayEffectSpecToOwner _returnvalue)
    (Abilities|TryActivateAbilitybyClass (Ability|GetAbilitySystemComponentfromActorInfo) "/Game/Game/Blueprints/GamePlayAbilities/GA_TalentArtRecast.GA_TalentArtRecast_C" true)
    (else
      (Variables|Default|SetCooldownDuration (Utilities|Struct|MakeScalableFloat (Variables|Default|GetRecastSecond)))
      (Variables|Default|SetTalentArtFlag false)
      (bind _returnvalue_2 (Class|AbilitySystemBlueprintLibrary|AddGrantedTags (GameplayEffects|MakeOutgoingSpec :self (Ability|GetAbilitySystemComponentfromActorInfo) :GameplayEffectClass "/Game/Game/Blueprints/GamePlayEffects/GE_ArtRecastStandby.GE_ArtRecastStandby_C") (Variables|Default|GetCooldownTags)))
      (Variables|Default|SetCooldownStandbyEffectSpec _returnvalue_2))))

(event EventChoose
  (params (Member :type Actor%20Object%20Reference))
  ;[0.15 0.15 0.15 0.5] アーツ対象選択処理
  ;;[0.15 0.15 0.15 0.5] メンバー選択処理
  (Utilities|Array|Add (Variables|Default|GetTargetList) Member)
  (CallFunction|AnimationStart))

(event EventCancelSelect
  ;[0.15 0.15 0.15 0.5] アーツ対象選択処理
  ;;[0.15 0.15 0.15 0.5] メンバー選択処理
  (Ability|CancelAbility))

(fn JudgeArtUseable
  (bind _returnvalue (Ability|GetAvatarActorfromActorInfo))
  (if (Variables|Default|GetTalentArtFlag)
    (return (== (.ReturnValue (Ability|Attribute|GetFloatAttribute _returnvalue "(AttributeName=\"TalentArtGage\",Attribute=/Script/XenoLikeProject.XenoCharacterAttributeSet:TalentArtGage,AttributeOwner=\"/Script/CoreUObject.Class'/Script/XenoLikeProject.XenoCharacterAttributeSet'\")")) (.ReturnValue (Ability|Attribute|GetFloatAttribute _returnvalue "(AttributeName=\"TalentArtGageMax\",Attribute=/Script/XenoLikeProject.XenoCharacterAttributeSet:TalentArtGageMax,AttributeOwner=\"/Script/CoreUObject.Class'/Script/XenoLikeProject.XenoCharacterAttributeSet'\")"))))
    (else
      (bind _returnvalue_2 (Ability|CommitAbilityCost false))
      (return _returnvalue_2))))

(fn IsSameType
  (params (Character1 :type Actor%20Object%20Reference) (Character2 :type Actor%20Object%20Reference) (Inverse :type Boolean))
  (bind _type (Class|BPICharacter|GetCharacterType(Message) Character1))
  (bind _type_2 (Class|BPICharacter|GetCharacterType(Message) Character2))
  (return (!= (Utilities|Enum|Equal(Enum) _type_2 _type) Inverse)))

(fn IsTargetHitable
  (params (Target :type Actor%20Object%20Reference))
  (bind _output_get (LocalVariables|SetLTarget Target))
  (bind _result (Class|BPICharacter|GetIsDeath(Message) _output_get))
  (if (not _result)
    (bind _status (Class|BPIXenoGameMode|IsinChainAttack(Message) (Game|GetGameMode)))
    (if _status
      (bind _returnvalue (Class|PartySubsystem|GetPartyMembers (Subsystems|GetPartySubsystem)))
      (bind _asbp_xeno_project_character (Utilities|Casting|CastToBP_XenoProjectCharacter (LocalVariables|GetLTarget)))
      (if (< (Utilities|Array|FindItem _returnvalue _asbp_xeno_project_character) 0)
        (if (>= (Utilities|Array|FindItem (Variables|/Script/XenoLikeProject.EnemiesSubsystem|GetEnemies (Subsystems|GetEnemiesSubsystem)) (LocalVariables|GetLTarget)) 0)
          (return true)
          (else
            (return false)))
        (else
          (return true)))
      (else
        (return true)))
    (else
      (return false))))

(fn GetRecastTime
  (return (Variables|Default|GetRecastSecond)))