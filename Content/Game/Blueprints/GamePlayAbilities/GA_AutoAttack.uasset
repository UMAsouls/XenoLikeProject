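; Gameplay ability for a character's auto-attack against its current lock-on target.
; It checks cost and attack eligibility, faces the target, then plays a montage at the avatar's attack speed.
; A gameplay event during the montage triggers a BP_AttackHitStrategy hit check; hits play a sound and apply GE_AutoAttack.
; Cooldown duration comes from the avatar and is committed only on a hit.
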(event Custom|SetCooldownTime
  (bind _cooldowntime (Class|BPICharacter|GetAutoAttackCooldownTime(Message) (Ability|GetAvatarActorfromActorInfo)))
  (Variables|Default|SetCooldownDuration (Utilities|Struct|MakeScalableFloat _cooldowntime)))

(event Ability|EventActivateAbility
  (bind _returnvalue (Ability|GetAvatarActorfromActorInfo))
  (bind _returnvalue_2 (Ability|CommitAbilityCost false))
  (if _returnvalue_2
    (CallFunction|SetCooldownTime)
    (bind _status (Class|BPICharacter|AutoAttackAble(Message) (Ability|GetAvatarActorfromActorInfo)))
    (if _status
      (Class|BPICharacter|LookatLockonTarget(Message) (Ability|GetAvatarActorfromActorInfo))
      (bind _speed (Class|BPICharacter|GetAutoAttackSpeed(Message) (Ability|GetAvatarActorfromActorInfo)))
      (|PlayMontageandWaitProxy "None" (Variables|Default|GetMontage%20to%20Play) _speed "None" true 1.0 0.0 false
        (:then
          (bind _asynctaskproxy (Ability|Tasks|WaitGameplayEvent (Variables|Default|GetEvent%20Tag) 0)
            (:then
              (Variables|Default|SetAttackEvent _asynctaskproxy))
            (:EventReceived
              (GameplayAttributes|GetAttributeSet (Ability|GetAbilitySystemComponentfromActorInfo) "/Script/XenoLikeProject.XenoCharacterAttributeSet")
              (bind _target (Class|BPICharacter|GetCurrentLockonTarget(Message) (Ability|GetAvatarActorfromActorInfo)))
              (Utilities|IsValid _target
                (:Is%20Valid
                  (bind _returnvalue_3 (Game|ConstructObjectfromClass "/Game/Game/Blueprints/GamePlayAbilities/ArtHitHandler/BP_AttackHitStrategy.BP_AttackHitStrategy_C"))
                  (bind _result (Default|JudgeHit _returnvalue_3 _returnvalue _target))
                  (if _result
                    (Audio|PlaySoundatLocation (Variables|Default|GetHitSound) (Transformation|GetActorLocation _returnvalue) "0, 0, 0" (Variables|Default|GetSoundVolume) 1.0 0.0 0 0 0 0)
                    (GameplayEffects|ApplyGameplayEffectSpecToTarget (GameplayEffects|MakeOutgoingSpec :self (Ability|GetAbilitySystemComponentfromActorInfo) :GameplayEffectClass "/Game/Game/Blueprints/GamePlayEffects/Battle/GE_AutoAttack.GE_AutoAttack_C") (Ability|TargetData|AbilityTargetDatafromActor _target))
                    (Ability|CommitAbilityCooldown false)))))))
        (:OnCompleted
          (Ability|EndAbility))
        (:OnInterrupted
          (Ability|CancelAbility)))
      (else
        (Ability|CancelAbility)))
    (else
      (Ability|CancelAbility))))

(event Ability|EventOnEndAbility
  (params (bWasCancelled :type Boolean))
  (Utilities|IsValid (Variables|Default|GetAttackEvent)
    (:Is%20Valid
      (GameplayTasks|EndTask (Variables|Default|GetAttackEvent)))))