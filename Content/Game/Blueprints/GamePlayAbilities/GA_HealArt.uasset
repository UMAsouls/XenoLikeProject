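; GA_HealArt is a gameplay ability for a healing art cast on a battle member chosen by the player.
; Activation commits the cost and asks the player controller to start member selection, which calls back Choose or CancelSelect.
; Choose applies a move-stop effect to the caster and plays a montage, whose hit event applies GE_HealArt to the target with a SetByCaller heal bonus.
; Cooldown is committed when the montage completes.
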(event Ability|EventActivateAbility
  (bind _returnvalue (Ability|CommitAbilityCost false))
  (if _returnvalue
    (Class|BPICharacterController|BattleMemberSelectStart(Message) (Game|GetPlayerController 0) self)
    (else
      (Ability|EndAbility))))

(event Ability|EventOnEndAbility
  (params (bWasCancelled :type Boolean))
  (bind _async_task (Variables|Default|GetAsync%20Task))
  (|CallParentFunction bWasCancelled)
  (Utilities|IsValid _async_task
    (:Is%20Valid
      (GameplayTasks|EndTask _async_task))))

(event EventCancelSelect
  (Ability|CancelAbility))

(event EventChoose
  (params (Member :type Actor%20Object%20Reference))
  (Ability|ApplyGameplayEffectToOwner "/Game/Game/Blueprints/GamePlayEffects/Battle/GE_MoveStop.GE_MoveStop_C")
  (Variables|Default|SetTarget Member)
  (|PlayMontageandWaitProxy "None" (Variables|Default|GetMontage%20to%20Play) 1.0 "None" true 1.0 0.0 false
    (:then
      (bind _asynctaskproxy (Ability|Tasks|WaitGameplayEvent "(TagName=\"Event.Montage.Attack.Hit\")" 0)
        (:then
          (Variables|Default|SetAsync%20Task _asynctaskproxy))
        (:EventReceived
          (Utilities|IsValid (Variables|Default|GetTarget)
            (:Is%20Valid
              (bind _returnvalue (Ability|GameplayEffect|AssignTagSetbyCallerMagnitude (GameplayEffects|MakeOutgoingSpec :self (Ability|GetAbilitySystemComponent (Ability|GetAvatarActorfromActorInfo)) :GameplayEffectClass "/Game/Game/Blueprints/GamePlayEffects/GE_HealArt.GE_HealArt_C") "(TagName=\"Effect.Heal.ArtBonus\")" (Variables|Default|GetHealBonus)))
              (GameplayEffects|ApplyGameplayEffectSpecToTarget _returnvalue (Ability|TargetData|AbilityTargetDatafromActor (Variables|Default|GetTarget))))))))
    (:OnCompleted
      (Ability|EndAbility)
      (Ability|CommitAbilityCooldown false))))