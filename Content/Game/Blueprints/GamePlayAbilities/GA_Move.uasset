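; GA_Move is a gameplay ability that represents character movement as an active ability so gameplay tags can govern whether movement is allowed.
; On activation it schedules a next-tick check that asks the avatar whether a move is being called.
; While one is, it calls the avatar's moving message and schedules another next-tick timer to stay active, otherwise it ends.
; Ending the ability clears the pending timer.
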(event Custom|MoveCheck
  ;[0.15 0.15 0.15 0.5] 移動中はずっとアビリティ発動状態にするための処理
  (bind _status (Class|BPIControlCharacter|IsMoveCalling(Message) (Ability|GetAvatarActorfromActorInfo)))
  (if _status
    (Class|BPIPlayer|CallMoving(Message) (Ability|GetAvatarActorfromActorInfo))
    (bind _returnvalue (Class|KismetSystemLibrary|SetTimerforNextTickDelegate (EventDispatchers|CreateEvent :!event Custom|MoveCheck)))
    (Variables|Default|SetTimerHandle _returnvalue)
    (else
      (Ability|EndAbility))))

(event Ability|EventActivateAbility
  ;[0.15 0.15 0.15 0.5] Abilityで移動管理することで、移動可否をtag管理
  (bind _returnvalue (Class|KismetSystemLibrary|SetTimerforNextTickDelegate (delegate Custom|MoveCheck)))
  (Variables|Default|SetTimerHandle _returnvalue))

(event Ability|EventOnEndAbility
  (params (bWasCancelled :type Boolean))
  (Utilities|Time|ClearandInvalidateTimerbyHandle (Variables|Default|GetTimerHandle)))