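; GA_SingleAttackArt is a Gameplay Ability for an attack art that hits the avatar's current lock-on target.
; On hit, it runs the parent logic, then gets the target from the avatar through an interface message.
; If the target is valid, it applies a GE_Attack spec to it, passing DamageBonus as a SetByCaller magnitude under the Effect.Damage.ArtBonus tag.
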(event EventOnHit
  (|CallParentFunction)
  (bind _target (Class|BPICharacter|GetCurrentLockonTarget(Message) (Ability|GetAvatarActorfromActorInfo)))
  (Utilities|IsValid _target
    (:Is%20Valid
      (bind _returnvalue (Ability|GameplayEffect|AssignTagSetbyCallerMagnitude (GameplayEffects|MakeOutgoingSpec :self (Ability|GetAbilitySystemComponent (Ability|GetAvatarActorfromActorInfo)) :GameplayEffectClass "/Game/Game/Blueprints/GamePlayEffects/Battle/GE_Attack.GE_Attack_C") "(TagName=\"Effect.Damage.ArtBonus\")" (Variables|Default|GetDamageBonus)))
      (GameplayEffects|ApplyGameplayEffectSpecToTarget _returnvalue (Ability|TargetData|AbilityTargetDatafromActor _target)))))