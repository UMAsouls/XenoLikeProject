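; GA_TalentArtRecast is a Gameplay Ability that manages the recast cooldown of a Talent Art.
; On activation it applies a start effect, then a recast effect granting the Talent cooldown tag, and stores that effect's handle.
; It repeatedly waits for attribute changes until two avatar attribute values are equal, then ends.
; Ending the ability removes the recast effect through the stored handle.
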(event Ability|EventActivateAbility
  (bind _returnvalue (Ability|GetAvatarActorfromActorInfo))
  (Ability|ApplyGameplayEffectToOwner "/Game/Game/Blueprints/GamePlayEffects/GE_TalentArtRecastStart.GE_TalentArtRecastStart_C")
  (bind _returnvalue_2 (Class|AbilitySystemBlueprintLibrary|AddGrantedTags (GameplayEffects|MakeOutgoingSpec :self (Ability|GetAbilitySystemComponentfromActorInfo) :GameplayEffectClass "/Game/Game/Blueprints/GamePlayEffects/GE_TalentArtRecast.GE_TalentArtRecast_C") "(GameplayTags=((TagName=\"Art.Cooldown.Talent\")))"))
  (bind _returnvalue_3 (Ability|ApplyGameplayEffectSpecToOwner _returnvalue_2))
  (Variables|Default|SetActiveCooldownEffectSpecHandle _returnvalue_3)
  (|WaitforAttributeChange :Attribute "(AttributeName=\"TalentArtGage\",Attribute=/Script/XenoLikeProject.XenoCharacterAttributeSet:TalentArtGage,AttributeOwner=\"/Script/CoreUObject.Class'/Script/XenoLikeProject.XenoCharacterAttributeSet'\")" :OptionalExternalOwner 0 :!label _label
    (:OnChange
      (if (== (.ReturnValue (Ability|Attribute|GetFloatAttribute _returnvalue "(AttributeName=\"TalentArtGage\",Attribute=/Script/XenoLikeProject.XenoCharacterAttributeSet:TalentArtGage,AttributeOwner=\"/Script/CoreUObject.Class'/Script/XenoLikeProject.XenoCharacterAttributeSet'\")")) (.ReturnValue (Ability|Attribute|GetFloatAttribute _returnvalue "(AttributeName=\"TalentArtGageMax\",Attribute=/Script/XenoLikeProject.XenoCharacterAttributeSet:TalentArtGageMax,AttributeOwner=\"/Script/CoreUObject.Class'/Script/XenoLikeProject.XenoCharacterAttributeSet'\")")))
        (Ability|EndAbility)
        (else
          (goto _label))))))

(event Ability|EventOnEndAbility
  (params (bWasCancelled :type Boolean))
  (Ability|RemoveGameplayEffectFromOwnerWithHandle (Variables|Default|GetActiveCooldownEffectSpecHandle)))