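; A VFX spawn-place strategy for gameplay abilities that places a single effect in front of the source actor.
; It offsets the source's location along its forward vector by SpawnDistance, then lowers it by the capsule's scaled half-height, toward foot level.
; The returned transform keeps the source's rotation at unit scale and ignores the targets.
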(fn CalculateSpawnPlace
  (params (Targets :type Array%20of%20Actor%20Object%20References) (Source :type Actor%20Object%20Reference))
  (return (Utilities|Array|MakeArray (Math|Transform|MakeTransform (- (+ (Transformation|GetActorLocation Source) (* (Transformation|GetActorForwardVector Source) (LocalVariables|GetSpawnDistance))) (Math|Vector|MakeVector 0.0 0.0 (Components|Capsule|GetScaledCapsuleHalfHeight (Actor|GetComponentbyClass Source "/Script/Engine.CapsuleComponent")))) (Transformation|GetActorRotation Source)))))