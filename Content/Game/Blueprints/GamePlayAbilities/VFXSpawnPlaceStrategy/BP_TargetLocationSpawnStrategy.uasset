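; BP_TargetLocationSpawnStrategy is a VFX spawn placement strategy for gameplay abilities that computes a spawn transform at each target's location.
; CalculateSpawnPlace loops over the targets and lowers each actor location by its capsule component's scaled half height, placing the point at the capsule's base.
; It returns these transforms with zero rotation and unit scale, and does not use the Source input.
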(fn CalculateSpawnPlace
  (params (Targets :type Array%20of%20Actor%20Object%20References) (Source :type Actor%20Object%20Reference))
  (for _array_element Targets
    (Utilities|Array|Add (LocalVariables|GetTransforms) (Math|Transform|MakeTransform (- (Transformation|GetActorLocation _array_element) (Math|Vector|MakeVector 0.0 0.0 (Components|Capsule|GetScaledCapsuleHalfHeight (Actor|GetComponentbyClass _array_element "/Script/Engine.CapsuleComponent")))))))
  (return (LocalVariables|GetTransforms)))